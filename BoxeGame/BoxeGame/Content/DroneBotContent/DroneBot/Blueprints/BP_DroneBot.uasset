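; BP_DroneBot is a physics-constrained drone that reacts to hits like a punch bag.
; A hit on SM_Drone stops a timeline, resets the constraint's angular drive to low stiffness and high damping, plays a sound, spawns Niagara fireworks near the other component, and calls OnPunchBag.
; An overlap on the drone plays a timeline that blends the drive's position and velocity strengths, tuning its springiness over time.
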(event OnComponentBeginOverlap(SM_Drone)
  (params (OverlappedComponent :type Primitive%20Component%20Object%20Reference) (OtherActor :type Actor%20Object%20Reference) (OtherComp :type Primitive%20Component%20Object%20Reference) (OtherBodyIndex :type Integer) (bFromSweep :type Boolean) (SweepResult :type Hit%20Result%20Structure%20%28by%20ref%29))
  (Utilities|FlowControl|Sequence
    (:then_0
      (bind _alpha (Timeline|Timeline_0 PlayFromStart)
        (:Update
          (Class|PhysicsConstraintComponent|SetAngularDriveParams (Variables|Default|GetPhysicsConstraint) (Math|Float|Lerp (Math|Float|MakeLiteralFloat 1e+02) 4e+02 _alpha) (Math|Float|Lerp (Math|Float|MakeLiteralFloat 3e+01) 1.0 _alpha) 0.0))))))

(event OnComponentHit(SM_Drone)
  (params (HitComponent :type Primitive%20Component%20Object%20Reference) (OtherActor :type Actor%20Object%20Reference) (OtherComp :type Primitive%20Component%20Object%20Reference) (NormalImpulse :type Vector :default "0, 0, 0") (Hit :type Hit%20Result%20Structure%20%28by%20ref%29))
  (bind _returnvalue (Transformation|GetWorldLocation OtherComp))
  (bind _sphere (Variables|Default|GetSphere))
  (bind _returnvalue_2 (Transformation|GetWorldLocation _sphere))
  (bind _returnvalue_3 (- _returnvalue_2 _returnvalue))
  (bind _returnvalue_4 (Math|Vector|Normalize _returnvalue_3))
  (bind _returnvalue_5 (* _returnvalue_4 5e+01))
  (bind _returnvalue_6 (+ _returnvalue _returnvalue_5))
  (Utilities|FlowControl|Sequence
    (:then_0
      (Audio|Components|Audio|Stop (Variables|Default|GetTimeline_0))
      (Class|PhysicsConstraintComponent|SetAngularDriveParams (Variables|Default|GetPhysicsConstraint) (Math|Float|MakeLiteralFloat 3e+01) (Math|Float|MakeLiteralFloat 1e+02) 0.0)
      (Audio|PlaySoundatLocation "/Game/Project/Sounds/hit.hit" (Transformation|GetWorldLocation OtherComp) "0, 0, 0" 1.0 1.0 0.0 0 0 0)
      (Niagara|SpawnSystematLocation "/Game/NiagaraAbstractSpace3/Effects/NS_Sphere_of_Fireworks.NS_Sphere_of_Fireworks" (Math|Vector|MakeVector (.x _returnvalue_6) (.y _returnvalue_6) (.z (Transformation|GetWorldLocation OtherComp)))))
    (:then_1
      (Default|CallOnPunchBag))))

(event EventBeginPlay)

(event Collision|EventActorBeginOverlap
  (params (OtherActor :type Actor%20Object%20Reference)))

(event EventTick
  (params (DeltaSeconds :type Float%20%28single-precision%29)))

(fn ConstructionScript)