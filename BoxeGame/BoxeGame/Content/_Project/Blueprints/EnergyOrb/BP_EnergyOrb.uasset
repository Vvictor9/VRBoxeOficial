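; BP_EnergyOrb is an orb that flies toward a fixed world location and applies a punch-value penalty to the VR pawn it hits.
; After a random start delay, a timeline lerps it from its current position each update toward that point, offset randomly along X.
; Any sphere overlap destroys the orb, and a VRPawn overlap also sends minus one point to the pawn's BPCTimer through AddPunchValue.
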(event OnComponentBeginOverlap(SphereCollision)
  (params (OverlappedComponent :type Primitive%20Component%20Object%20Reference) (OtherActor :type Actor%20Object%20Reference) (OtherComp :type Primitive%20Component%20Object%20Reference) (OtherBodyIndex :type Integer) (bFromSweep :type Boolean) (SweepResult :type Hit%20Result%20Structure%20%28by%20ref%29))
  (Utilities|FlowControl|Sequence
    (:then_0
      (Actor|DestroyActor))
    (:then_1
      (bind _asvrpawn (Utilities|Casting|CastToVRPawn OtherActor))
      (Default|AddPunchValue (Variables|/Game/_Project/Blueprints/VRPawn.VRPawn_C|GetBPC_Timer _asvrpawn) -1.0 0.0))))

(event EventBeginPlay
  (bind _returnvalue (+ "720.000000,140.000000,170.000000" "0, 0, 0"))
  (Utilities|FlowControl|Delay (Math|Random|RandomFloatinRange 0.0 3.0))
  (Variables|Default|SetRandomSide (Math|Random|RandomFloatinRange -5e+01 5e+01))
  (bind _alpha (Timeline|TL_MoveEnergyOrb PlayFromStart)
    (:Update
      (Transformation|SetActorLocation (Math|Vector|Lerp(Vector) (Transformation|GetActorLocation) (Math|Vector|MakeVector (+ (.x _returnvalue) (Variables|Default|GetRandomSide)) (.y _returnvalue) (.z _returnvalue)) _alpha) false false))))

(event Collision|EventActorBeginOverlap
  (params (OtherActor :type Actor%20Object%20Reference)))

(event EventTick
  (params (DeltaSeconds :type Float%20%28single-precision%29)))

(fn ConstructionScript)