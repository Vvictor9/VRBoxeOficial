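; BP_ProjectilePlacebo is a projectile that scores punch points for the VR player when its capsule overlaps a component named "Overlap".
; On that hit it activates the thunder hit effect, disables capsule collision, hides the shot effect and destroys itself after a short delay.
; In parallel, it casts the player pawn to VRPawn and adds punch value through that pawn's BPCTimer.
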(event OnComponentBeginOverlap(Capsule)
  (params (OverlappedComponent :type Primitive%20Component%20Object%20Reference) (OtherActor :type Actor%20Object%20Reference) (OtherComp :type Primitive%20Component%20Object%20Reference) (OtherBodyIndex :type Integer) (bFromSweep :type Boolean) (SweepResult :type Hit%20Result%20Structure%20%28by%20ref%29))
  (if (Utilities|Enum|Equal(Enum) (Utilities|GetObjectName OtherComp) "Overlap")
    (Utilities|FlowControl|Sequence
      (:then_0
        (Components|Activation|SetActive (Variables|Default|GetP_ky_hit_thunder) true true)
        (Collision|SetCollisionEnabled (Variables|Default|GetCapsule) "NoCollision")
        (Rendering|SetVisibility (Variables|Default|GetP_ky_shot_thunder) false false)
        (Utilities|FlowControl|Delay 1.0)
        (Actor|DestroyActor))
      (:then_1
        (bind _asvrpawn (Utilities|Casting|CastToVRPawn (Game|Player|GetPlayerPawn 0)))
        (Default|AddPunchValue (Variables|/Game/_Project/Blueprints/VRPawn.VRPawn_C|GetBPC_Timer _asvrpawn) 5.0 5.0)))))

(fn ConstructionScript)