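; Thunder projectile fired at the VR player, who punches it for points or loses points when hit.
; It scales up on spawn, then Shot enables collision, faces the camera and waits randomly before launching.
; A timeline lerps it toward just ahead of the live camera position, sometimes offset along world X.
; On overlap it plays a hit effect, scores punch-channel hits by hand speed via BPCTimer, penalizes other pawn hits, and self-destroys.
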(event OnComponentBeginOverlap(Capsule)
  (params (OverlappedComponent :type Primitive%20Component%20Object%20Reference) (OtherActor :type Actor%20Object%20Reference) (OtherComp :type Primitive%20Component%20Object%20Reference) (OtherBodyIndex :type Integer) (bFromSweep :type Boolean) (SweepResult :type Hit%20Result%20Structure%20%28by%20ref%29))
  (bind _returnvalue (Collision|GetCollisionObjectType OtherComp))
  (bind _returnvalue_2 (Utilities|Enum|Equal(Enum) _returnvalue "ECC_GameTraceChannel4"))
  (Utilities|FlowControl|Sequence
    (:then_0
      (Components|Activation|SetActive (Variables|Default|GetP_ky_hit_thunder) true true)
      (Collision|SetCollisionEnabled (Variables|Default|GetCapsule) "NoCollision")
      (Rendering|SetVisibility (Variables|Default|GetP_ky_shot_thunder) false false)
      (Utilities|FlowControl|Delay 1.0)
      (Actor|DestroyActor))
    (:then_1
      (bind _asvrpawn (Utilities|Casting|CastToVRPawn OtherActor))
      (if (or _returnvalue_2 (Utilities|Enum|Equal(Enum) _returnvalue "ECC_GameTraceChannel2"))
        (Default|AddPunchValue (Variables|/Game/_Project/Blueprints/VRPawn.VRPawn_C|GetBPC_Timer _asvrpawn) (/ (Math|Float|SelectFloat (Variables|/Game/_Project/Blueprints/VRPawn.VRPawn_C|GetPunchLSpeedValue _asvrpawn) (Variables|/Game/_Project/Blueprints/VRPawn.VRPawn_C|GetPunchRSpeedValue _asvrpawn) _returnvalue_2) 3.0) (/ (Math|Float|SelectFloat (Variables|/Game/_Project/Blueprints/VRPawn.VRPawn_C|GetPunchLSpeedValue _asvrpawn) (Variables|/Game/_Project/Blueprints/VRPawn.VRPawn_C|GetPunchRSpeedValue _asvrpawn) _returnvalue_2) 3.0))
        (else
          (Default|AddPunchValue (Variables|/Game/_Project/Blueprints/VRPawn.VRPawn_C|GetBPC_Timer _asvrpawn) -1e+02 0.0))))))

(event Custom|Shot
  (bind _asvrpawn (Utilities|Casting|CastToVRPawn (Game|Player|GetPlayerPawn 0)))
  (Collision|SetCollisionEnabled (Variables|Default|GetCapsule) "QueryOnly")
  (Transformation|SetActorRotation (Math|Rotator|FindLookatRotation (Transformation|GetActorLocation) (Transformation|GetWorldLocation (Variables|/Game/_Project/Blueprints/VRPawn.VRPawn_C|GetCamera _asvrpawn))) true)
  (Utilities|FlowControl|Delay (Math|Random|RandomFloatinRange 0.1 1.0))
  (if (== (Math|Random|RandomIntegerinRange 0 1) 0)
    (Variables|Default|SetDirection (Math|Vector|MakeVector (Math|Random|RandomFloatinRange -4e+01 4e+01) 0.0 0.0))
    (else
      (Variables|Default|SetDirection (Math|Vector|MakeVector 0.0 0.0 (Math|Random|RandomFloatinRange 0.0 0.0)))))
  (CallFunction|ProjectilMovement))

(event Custom|ProjectilMovement
  (bind _asvrpawn (Utilities|Casting|CastToVRPawn (Game|Player|GetPlayerPawn 0)))
  (bind _alpha (Timeline|Tl_ProjectileMovement PlayFromStart)
    (:Update
      (Transformation|SetActorLocation (Math|Vector|Lerp(Vector) (Transformation|GetActorLocation) (+ (+ (Transformation|GetWorldLocation (Variables|/Game/_Project/Blueprints/VRPawn.VRPawn_C|GetCamera _asvrpawn)) (Math|Vector|GetForwardVector (Variables|/Game/_Project/Blueprints/VRPawn.VRPawn_C|GetCamera _asvrpawn))) (Variables|Default|GetDirection)) _alpha) false false))
    (:Finished
      (Variables|Default|SetDirection "0, 0, 0"))))

(event EventBeginPlay
  (Transformation|SetActorScale3D "0, 0, 0")
  (Variables|/Script/Engine.ProjectileMovementComponent|SetHomingTargetComponent (Variables|Default|GetProjectileMovement) (Variables|/Script/Engine.Actor|GetRootComponent (Game|Player|GetPlayerPawn 0)))
  (Utilities|FlowControl|Sequence
    (:then_1
      (bind _scale (Timeline|Grow PlayFromStart)
        (:Update
          (Transformation|SetActorScale3D (Math|Vector|Lerp(Vector) "0, 0, 0" "1.000000,1.000000,1.000000" _scale)))))))

(fn ConstructionScript)