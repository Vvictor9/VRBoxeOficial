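; VR HUD actor that hosts the new-record widget, where the player enters a name after a record-breaking round.
; On round end it checks the save game for a record, then shows the start panel and score widget and enables VR pawn widget interaction.
; Saving or starting a round hides the widget and disables interaction.
; That close also saves the rank, defaulting to "Anonymous", through a DoOnce reset on each show.
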(event Custom|CheckIfHasNewRecord
  (params (ScoreValue :type Integer) (ScoreAbsolut :type Integer))
  (if (Default|IsNewRecord? (Variables|/Game/_Project/Framework/BP_GameInstance.BP_GameInstance_C|GetSaveGame (CallFunction|GetBoxegameInstance)) ScoreValue)
    (CallFunction|ShowNewRecord ScoreValue ScoreAbsolut)
    (bind _asvrpawn (Utilities|Casting|CastToVRPawn (Game|Player|GetPlayerPawn 0)))
    (Default|ActiveWidgetInteraction _asvrpawn true)))

(event Custom|CloseNewScore
  (bind _wdgetref (Variables|Default|GetWdgetRef))
  (bind _editabletextbox_68 (Variables|/Game/_Project/UI/WB_NewRecord.WB_NewRecord_C|GetEditableTextBox_68 _wdgetref))
  (bind _returnvalue (Class|EditableTextBox|GetText _editabletextbox_68))
  (bind _asvrpawn (Utilities|Casting|CastToVRPawn (Game|Player|GetPlayerPawn 0)))
  (Default|ActiveWidgetInteraction _asvrpawn false)
  (Widget|SetVisibility _wdgetref "Hidden")
  (Utilities|FlowControl|DoOnce false
    (:Completed
      (Default|SaveNewRank (CallFunction|GetBoxegameInstance) (Variables|Default|GetTotal%20Score) (select (Utilities|Text|TextIsEmpty _returnvalue) "Anonymous" _returnvalue) (Variables|Default|GetScoreAbsolut))
      (EventDispatchers|UnbindEventfromOnSaveScore (Variables|Default|GetWdgetRef) (delegate Custom|CloseNewScore)))))

(event Custom|ShowNewRecord
  (params (TotalScore :type Integer) (ScoreAbsolut :type Integer))
  (bind _wdgetref (Variables|Default|GetWdgetRef))
  (bind _wdgetref_2 (Variables|Default|GetWdgetRef))
  (bind _editabletextbox_68 (Variables|/Game/_Project/UI/WB_NewRecord.WB_NewRecord_C|GetEditableTextBox_68 _wdgetref))
  (bind _returnvalue (Class|EditableTextBox|GetText _editabletextbox_68))
  (Variables|Default|SetTotal%20Score TotalScore)
  (Variables|Default|SetScoreAbsolut ScoreAbsolut)
  (bind _outactors (Actor|GetAllActorsOfClass "/Game/_Project/Blueprints/BP_StartPanel.BP_StartPanel_C"))
  (Default|ShowPanel (Utilities|Array|Get(acopy) _outactors))
  (Default|UpdateScore _wdgetref_2 (Variables|Default|GetTotal%20Score))
  (Widget|SetVisibility _wdgetref_2 "Visible")
  (EventDispatchers|BindEventtoOnSaveScore _wdgetref_2 (delegate Custom|CloseNewScore))
  (Utilities|FlowControl|DoOnce false) ; enters at Reset
)

(event EventBeginPlay
  (bind _aswb_new_record (Utilities|Casting|CastToWB_NewRecord (UserInterface|GetWidget (Variables|Default|GetWidget)) :!label _label)
    (:then
      (Variables|Default|SetWdgetRef _aswb_new_record)
      (EventDispatchers|BindEventtoOnEndRound (CallFunction|GetBoxegameInstance) (delegate Custom|CheckIfHasNewRecord))
      (Widget|SetVisibility (Variables|Default|GetWdgetRef) "Hidden")
      (EventDispatchers|BindEventtoOnStartRound (CallFunction|GetBoxegameInstance) (delegate Custom|CloseNewScore)))
    (:CastFailed
      (Utilities|FlowControl|Delay 1.0)
      (goto _label))))

(fn ConstructionScript)