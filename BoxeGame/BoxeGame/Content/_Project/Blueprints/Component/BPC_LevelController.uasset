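; Level controller component that moves the VR player to the next map in a list behind a fade-to-black.
; ChangeToNextLevel spawns a scaled-up BP_Sphere at the VR pawn and starts a looping timer.
; Each tick raises the opacity of a dynamic sphere material created at BeginPlay.
; Past the alpha threshold, it destroys the sphere, advances the wrapping map index and opens that level as a listen server.
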(event Custom|ChangeToNextLevel
  (bind _returnvalue (Game|SpawnActorfromClass "/Game/_Project/Blueprints/BP_Sphere.BP_Sphere_C" (Math|Transform|MakeTransform (Transformation|GetActorLocation (Variables|Default|GetVRPawnRef)) "0, 0, 0" "3.000000,3.000000,3.000000") "Undefined" 0 0))
  (Variables|Default|SetSphereRef _returnvalue)
  (bind _returnvalue_2 (Utilities|Time|SetTimerbyEvent (delegate Custom|FadeToBlack) 0.1 true))
  (Variables|Default|SetTH_IncrementAlpha _returnvalue_2))

(event Custom|FadeToBlack
  (bind _output_get (Variables|Default|SetAlpha (+ (Variables|Default|GetAlpha) 0.02)))
  (if (> _output_get 1.5)
    (Math|Integer|IncrementInt (Variables|Default|GetMapIndex)
      (:%20%20
        (Actor|DestroyActor (Variables|Default|GetSphereRef))
        (if (== (Variables|Default|GetMapIndex) 4)
          (Variables|Default|SetMapIndex 0)
          (Utilities|Time|ClearandInvalidateTimerbyHandle (Variables|Default|GetTH_IncrementAlpha))
          (Game|OpenLevel(byName) (Utilities|Array|Get(acopy) (Variables|Default|GetMapsName) (Variables|Default|GetMapIndex)) true "?listen")
          (else
            (Game|OpenLevel(byName) (Utilities|Array|Get(acopy) (Variables|Default|GetMapsName) (Variables|Default|GetMapIndex)) true "?listen")))))
    (else
      (Rendering|Material|SetScalarParameterValue (Variables|Default|GetDMI_SphereFadeIn) "OpacityParam" _output_get :!class /Script/Engine.MaterialInstanceDynamic)
      (Rendering|Material|SetMaterial (Variables|/Game/_Project/Blueprints/BP_Sphere.BP_Sphere_C|GetSphere (Variables|Default|GetSphereRef)) 0 (Variables|Default|GetDMI_SphereFadeIn)))))

(event EventBeginPlay
  (bind _asvrpawn (Utilities|Casting|CastToVRPawn (Game|Player|GetPlayerPawn 0)))
  (Variables|Default|SetVRPawnRef _asvrpawn)
  (bind _returnvalue (Rendering|Material|CreateDynamicMaterialInstance "/Game/_Project/Material/M_Sphere.M_Sphere" "None" "None" :!class /Script/Engine.KismetMaterialLibrary))
  (Variables|Default|SetDMI_SphereFadeIn _returnvalue))