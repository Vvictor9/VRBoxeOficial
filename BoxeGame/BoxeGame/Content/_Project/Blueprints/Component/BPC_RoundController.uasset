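; Round controller component on the VR pawn that runs boxing rounds as alternating timed punch and rest sessions.
; Looping timers advance each phase, toggling punch scoring, recoloring the ring, spawning warning actors and driving the player HUD.
; Accepted punches add score and charge boosted mana.
; The game instance broadcasts round start and end, compares block scores and saves experience for four attributes (QuantaPulse, SurgeCore, AetherStream, EchoSense).
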(event Custom|EndRound
  (params (ScoreValue :type Integer) (ScoreAbsolut :type Integer))
  (Default|FinishRound (Variables|Default|GetWidgetRef))
  (Audio|PlaySound2D "/Game/_Project/Sounds/Alert_Cue.Alert_Cue" 1.0 1.0 0.0 0 0)
  (Input|EnableInput (Pawn|GetControlledPawn (Game|GetPlayerController 0)) (Game|GetPlayerController 0))
  (Variables|Default|SetSetIsInRoundMode? false))

(event EventBeginPlay
  (Utilities|FlowControl|Sequence
    (:then_0
      (if (Variables|/Game/_Project/Framework/BP_GameInstance.BP_GameInstance_C|GetIsDebug (CallFunction|GetBoxegameInstance))
        (Variables|Timer|SetMaxTimerPunch 5)
        (Variables|Timer|SetMaxTimerRest 5)
        (Variables|Timer|SetQuantSessionsInOneRound 2)))
    (:then_1
      (bind _asvrpawn (Utilities|Casting|CastToVRPawn (Components|GetOwner)))
      (Variables|Default|SetOwnerRef _asvrpawn)
      (bind _aswi_player_hud (Utilities|Casting|CastToWI_PlayerHUD (UserInterface|GetWidget (Variables|/Game/_Project/Blueprints/VRPawn.VRPawn_C|GetHUD _asvrpawn)) :!label _label)
        (:then
          (bind _output_get (Variables|Default|SetWidgetRef _aswi_player_hud))
          (Default|SetPunchValue _output_get)
          (bind _outactors (Actor|GetAllActorsOfClass "/Game/_Project/Blueprints/BP_AttributesHud.BP_AttributesHud_C"))
          (bind _aswb_character_attributes (Utilities|Casting|CastToWB_CharacterAttributes (UserInterface|GetWidget (Variables|/Game/_Project/Blueprints/BP_AttributesHud.BP_AttributesHud_C|GetWidget (Utilities|Array|Get(acopy) _outactors)))))
          (Variables|Default|Set%20WB%20Character%20Attributes%20Ref _aswb_character_attributes))
        (:CastFailed
          (Utilities|FlowControl|Delay 0.5)
          (goto _label))))
    (:then_2
      (EventDispatchers|BindEventtoOnEndRound (CallFunction|GetBoxegameInstance) (delegate Custom|EndRound)))))

(fn StartRound
  (CallFunction|ResetValues)
  (Variables|Default|SetSetIsInRoundMode? true)
  (Default|DroneHeightAdjustments (Variables|/Game/_Project/Blueprints/VRPawn.VRPawn_C|GetDroneBotRef (Variables|Default|GetOwnerRef)))
  (Utilities|Time|SetTimerbyFunctionName (Variables|Default|GetWidgetRef) "InitStartTimer" 3.0)
  (Utilities|Time|SetTimerbyEvent (EventDispatchers|CreateEvent :!event StartPunchTimer) 3.0)
  (Variables|Default|SetTimeToUnloading 0.0)
  (Default|CallOnStartRound (CallFunction|GetBoxegameInstance)))

(fn StartRestTimer
  (bind _widgetref (Variables|Default|GetWidgetRef))
  (bind _widgetref_2 (Variables|Default|GetWidgetRef))
  (Variables|Default|SetIsInResTime? true)
  (CallFunction|SpawnWarningActor "/Game/_Project/Blueprints/BP_WarningAtRest.BP_WarningAtRest_C" "(R=1.000000,G=0.000000,B=0.000000,A=1.000000)")
  (CallFunction|ChangeRingueColor "(R=1.000000,G=0.000000,B=0.000000,A=1.000000)")
  (Variables|Default|SetTimerCurrentValue 0)
  (CallFunction|BlockPunchCount)
  (Default|StartRestTime (Variables|Default|GetWidgetRef) (Variables|Timer|GetQuantPunchSessions))
  (bind _returnvalue (Utilities|Time|SetTimerbyEvent (EventDispatchers|CreateEvent :!event UpdateTimerRest) 1.0 true))
  (Variables|Default|SetTimer_Timer _returnvalue)
  (Default|SavePointsbyBlock (CallFunction|GetBoxegameInstance) (Variables|Timer|GetCurrentScoreInThisTime))
  (bind _pointsbetweenblocks (Default|ReturnPointsBetweenBlocks (CallFunction|GetBoxegameInstance) (Variables|Timer|GetCurrentScoreInThisTime) (Variables|Default|GetIsSecondTimerPunch)))
  (CallFunction|AddExptoAetherStream (Variables|Default|GetIsSecondTimerPunch) _pointsbetweenblocks)
  (Default|SetTxtPointsBetweenRound (Variables|Default|GetWidgetRef) _pointsbetweenblocks)
  (Default|InitLoadingBarTimer _widgetref (Variables|Default|GetDelayLoadingBarTimer))
  (Default|InitPBPunchTime _widgetref (Variables|Default|GetDelayPBPunchTime))
  (Audio|PlaySound2D "/Game/_Project/Sounds/Alert_Cue.Alert_Cue" 1.0 1.0 0.0 0 0)
  (Default|CallStartRestTime)
  (if (Variables|Default|GetIsSecondTimerPunch)
    (if (> (Variables|Timer|GetCurrentScoreInThisTime) (Variables|/Game/_Project/Blueprints/BP_SaveGame.BP_SaveGame_C|GetlastScoreAdd (Variables|/Game/_Project/Framework/BP_GameInstance.BP_GameInstance_C|GetSaveGame (CallFunction|GetBoxegameInstance))))
      (Default|SetAboveScoreVisibility _widgetref_2 true true)
      (else
        (Default|SetAboveScoreVisibility _widgetref_2 true false)))))

(fn StartPunchTimer
  (Development|SetHiddeninGame (Variables|/Game/_Project/Blueprints/VRPawn.VRPawn_C|GetP_ky_IceEffect_Left (Variables|Default|GetOwnerRef)) false false)
  (CallFunction|MakeManaBooster1 (Math|Conversions|ToFloat(Integer) (Utilities|Array|Get(acopy) (Variables|/Game/_Project/UI/WB_CharacterAttributes.WB_CharacterAttributes_C|GetLevelAttributes (Variables|Default|Get%20WB%20Character%20Attributes%20Ref)))))
  (CallFunction|DischargeMana 1.0)
  (Variables|/Game/_Project/Blueprints/VRPawn.VRPawn_C|Set%20TotalSpeedPunch (Variables|Default|GetOwnerRef) 0.0)
  (Variables|Default|SetIsInResTime? false)
  (CallFunction|SpawnWarningActor "/Game/_Project/Blueprints/BP_WarningInBattle.BP_WarningInBattle_C" "(R=1.000000,G=0.822786,B=0.009721,A=1.000000)")
  (CallFunction|ChangeRingueColor "(R=1.000000,G=0.822786,B=0.009721,A=1.000000)")
  (Audio|PlaySound2D "/Game/_Project/Sounds/Alert_Cue.Alert_Cue" 1.0 1.0 2.0 0 0)
  (Variables|Timer|SetCurrentScoreInThisTime 0)
  (Variables|Default|SetTimerCurrentValue 0)
  (Utilities|FlowControl|Sequence
    (:then_0
      (CallFunction|UnlockPunchCount false)
      (bind _returnvalue (Utilities|Time|SetTimerbyEvent (EventDispatchers|CreateEvent :!event UpdateTimerPunch) 1.0 true 4.0))
      (Variables|Default|SetTimer_Timer _returnvalue)
      (bind _returnvalue_2 (Utilities|Time|SetTimerbyEvent (EventDispatchers|CreateEvent :!event AddExptoQuantaPulse) 1.0 true 4.0))
      (Variables|Default|SetTH_ExpQuantaPulse _returnvalue_2)
      (bind _returnvalue_3 (Utilities|Time|SetTimerbyEvent (EventDispatchers|CreateEvent :!event AddExptoSurgeCore) 1.0 true (Variables|Default|GetInitial%20Start%20Delay)))
      (Variables|Default|SetTH_ExpSurgeCore _returnvalue_3)
      (if (Variables|Default|GetIsSecondTimerPunch)
        (bind _returnvalue_4 (Utilities|Time|SetTimerbyFunctionName (Variables|Default|GetWidgetRef) "InitUnloadingBarTimer" (Variables|Default|GetTimeToUnloading)))
        (Variables|Default|SetTHUnLoadingBarAnimation _returnvalue_4)
        (bind _returnvalue_5 (Utilities|Time|SetTimerbyFunctionName (Variables|Default|GetWidgetRef) "UnloadPBPunchTime" (Variables|Default|GetTimeToUnloading)))
        (Variables|Default|SetTHUnloadPBPunchTime _returnvalue_5)
        (else
          (bind _returnvalue_6 (Utilities|Time|SetTimerbyFunctionName (Variables|Default|GetWidgetRef) "InitUnloadingBarTimer" 4.0))
          (Variables|Default|SetTHUnLoadingBarAnimation _returnvalue_6)
          (bind _returnvalue_7 (Utilities|Time|SetTimerbyFunctionName (Variables|Default|GetWidgetRef) "UnloadPBPunchTime" 4.0))
          (Variables|Default|SetTHUnloadPBPunchTime _returnvalue_7))))
    (:then_1
      (Default|CallStartPunchTime))))

(fn UpdateTimerPunch
  (bind _output_get (Variables|Default|SetTimerCurrentValue (+ (Variables|Default|GetTimerCurrentValue) 1)))
  (if (>= _output_get (Variables|Timer|GetMaxTimerPunch))
    (CallFunction|StopPunchTime)))

(fn UpdateTimerRest
  (bind _maxtimerrest (Variables|Timer|GetMaxTimerRest))
  (bind _output_get (Variables|Default|SetTimerCurrentValue (+ (Variables|Default|GetTimerCurrentValue) 1)))
  (if (>= _output_get _maxtimerrest)
    (CallFunction|StopTimerRest)
    (CallFunction|AddExptoEchoSense (Default|ReturnEchoSenseValue (Variables|Default|GetOwnerRef)))
    (elif (>= _output_get (- _maxtimerrest 3))
      (Variables|Default|SetTimeToUnloading 3.0)
      (Default|StartPunchTime (Variables|Default|GetWidgetRef))
      (CallFunction|AddExptoEchoSense (Default|ReturnEchoSenseValue (Variables|Default|GetOwnerRef))))))

(fn StopTimerRest
  (Utilities|Time|ClearandInvalidateTimerbyHandle (Variables|Default|GetTimer_Timer))
  (Utilities|Time|ClearandInvalidateTimerbyHandle (Variables|Default|GetTHloadingBarAnimation))
  (CallFunction|BlockPunchCount)
  (Variables|Default|SetIsSecondTimerPunch true)
  (CallFunction|StartPunchTimer)
  (Default|SetAboveScoreVisibility (Variables|Default|GetWidgetRef) false false))

(fn StopPunchTime
  (Utilities|Time|ClearandInvalidateTimerbyHandle (Variables|Default|GetTimer_Timer))
  (Utilities|Time|ClearandInvalidateTimerbyHandle (Variables|Default|GetTHUnLoadingBarAnimation))
  (Utilities|Time|ClearandInvalidateTimerbyHandle (Variables|Default|GetTHUnloadPBPunchTime))
  (CallFunction|BlockPunchCount)
  (bind _output_get (Variables|Timer|SetQuantPunchSessions (+ (Variables|Timer|GetQuantPunchSessions) 1)))
  (if (>= _output_get (Variables|Timer|GetQuantSessionsInOneRound))
    (Default|CallOnEndRound (CallFunction|GetBoxegameInstance) (Variables|Default|GetScoreValue) (Variables|Default|GetScoreAbsolut))
    (else
      (CallFunction|StartRestTimer))))

(fn AddPunchValue
  (params (Points :type Float%20%28single-precision%29) (PointsToScoreAbsolut :type Float%20%28single-precision%29))
  (bind _returnvalue (Math|Float|Truncate Points))
  (if (not (Variables|Default|GetIsBlockingPunch))
    (bind _widgetref (Variables|Default|GetWidgetRef)
      (:then
        (bind _output_get (Variables|Default|SetScoreValue (+ (Variables|Default|GetScoreValue) _returnvalue)))
        (Variables|Default|SetScoreAbsolut (+ (Variables|Default|GetScoreAbsolut) (Math|Float|Truncate PointsToScoreAbsolut)))
        (Default|SetPunchValue _widgetref _output_get)
        (Variables|Timer|SetCurrentScoreInThisTime (+ (Variables|Timer|GetCurrentScoreInThisTime) _returnvalue))
        (CallFunction|ChargeMana (CallFunction|ReturnManatoCharge))
        (if (not (Variables|Default|GetCanBlockIncrement?))
          (Math|Float|IncrementFloat (Variables|Default|GetNumPunchsBySeocnds))))
      (:else))))

(fn BlockPunchCount
  (Variables|Default|SetIsBlockingPunch true))

(fn UnlockPunchCount
  (params (ResetValue :type Boolean))
  (Variables|Default|SetIsBlockingPunch false)
  (if ResetValue
    (Default|SetPunchValue (Variables|Default|GetWidgetRef) (Variables|Default|GetScoreValue))))

(fn SpawnWarningActor
  (params (ActorRef :type Actor%20Class%20Reference) (ColorRef :type Linear%20Color%20Structure))
  (Utilities|IsValid (Variables|Default|GetBP_WarningBattleRef)
    (:Is%20Valid
      (Actor|DestroyActor (Variables|Default|GetBP_WarningBattleRef)))
    (:Is%20Not%20Valid
      _))
  (bind _returnvalue (Game|SpawnActorfromClass ActorRef (Math|Transform|MakeTransform "717.376648,114.842361,25.000000") "Undefined" 0 0))
  (bind _output_get (Variables|Default|SetBP_WarningBattleRef _returnvalue))
  (bind _asbp_warning_in_battle (Utilities|Casting|CastToBP_WarningInBattle _output_get))
  (bind _returnvalue_2 (Rendering|Material|CreateDynamicMaterialInstance "/Game/_Project/Material/M_WarningLineInBattle.M_WarningLineInBattle" "None" "None" :!class /Script/Engine.KismetMaterialLibrary))
  (Rendering|Material|SetVectorParameterValue _returnvalue_2 "EmissiveColor" ColorRef :!class /Script/Engine.MaterialInstanceDynamic)
  (Rendering|Material|SetMaterial (Variables|/Game/_Project/Blueprints/BP_WarningInBattle.BP_WarningInBattle_C|GetSM_Warning _asbp_warning_in_battle) 0 _returnvalue_2))

(fn ChangeRingueColor
  (params (RingueRef :type Linear%20Color%20Structure))
  (bind _outactors (Actor|GetAllActorsOfClass "/Game/_Project/Blueprints/BP_Ringue.BP_Ringue_C"))
  (bind _returnvalue (Rendering|Material|CreateDynamicMaterialInstance "/Game/VRTemplate/Materials/M_Projectile.M_Projectile" "None" "None" :!class /Script/Engine.KismetMaterialLibrary))
  (Rendering|Material|SetVectorParameterValue _returnvalue "BaseColor" RingueRef :!class /Script/Engine.MaterialInstanceDynamic)
  (Rendering|Material|SetMaterial (Variables|/Game/_Project/Blueprints/BP_Ringue.BP_Ringue_C|GetSM_MERGED_ringue (Utilities|Array|Get(acopy) _outactors)) 0 _returnvalue))

(fn AddExptoQuantaPulse
  (bind _result (Math|Integer|IncrementInt (Variables|Default|GetSeconds))
    (:%20%20
      (if (== _result 5)
        (Variables|Default|SetBoosterToMana 1.0)
        (bind _quantapulsevalue (Default|ReturnQuantaPulseValue (Variables|Default|GetOwnerRef)))
        (Default|SaveAttributesProgress (CallFunction|GetBoxegameInstance) 0 _quantapulsevalue)
        (Default|UpdateQuantaPulseAttribute (Variables|Default|Get%20WB%20Character%20Attributes%20Ref))
        (Variables|Default|SetSeconds 10)
        (Development|SetHiddeninGame (Variables|/Game/_Project/Blueprints/VRPawn.VRPawn_C|GetP_ky_IceEffect_Left (Variables|Default|GetOwnerRef)) true false)
        (Utilities|Time|ClearandInvalidateTimerbyHandle (Variables|Default|GetTH_ExpQuantaPulse))))))

(fn AddExptoSurgeCore
  (bind _result (Math|Integer|IncrementInt (Variables|Default|GetSeconds))
    (:%20%20
      (if (== _result 16)
        (Default|SaveAttributesProgress (CallFunction|GetBoxegameInstance) 1 (Default|ReturnSurgeCoreValue (Variables|Default|GetOwnerRef) (Variables|Default|GetNumPunchsBySeocnds)))
        (Default|UpdateSurgeCoreAttribute (Variables|Default|Get%20WB%20Character%20Attributes%20Ref))
        (Variables|Default|SetCanBlockIncrement? true)
        (Variables|Default|SetNumPunchsBySeocnds 0.0)
        (Variables|Default|SetSeconds 0)
        (Utilities|Time|ClearandInvalidateTimerbyHandle (Variables|Default|GetTH_ExpSurgeCore))
        (else
          (Variables|Default|SetCanBlockIncrement? false)
          (CallFunction|MakeManaBooster1 0.0))))))

(fn AddExptoAetherStream
  (params (IsSecondTimerPunch :type Boolean) (ExpToAetherStream :type Integer))
  (if IsSecondTimerPunch
    (bind _aetherstreamcalculado (Default|ReturnAetherStreamValue (Variables|Default|GetOwnerRef) (Math|Conversions|ToFloat(Integer) ExpToAetherStream)))
    (Default|SaveAttributesProgress (CallFunction|GetBoxegameInstance) 2 _aetherstreamcalculado)
    (Default|UpdateAetherStreamAttribute (Variables|Default|Get%20WB%20Character%20Attributes%20Ref))
    (else
      (Default|SaveAttributesProgress (CallFunction|GetBoxegameInstance) 2 0.0)
      (Default|UpdateAetherStreamAttribute (Variables|Default|Get%20WB%20Character%20Attributes%20Ref)))))

(fn AddExptoEchoSense
  (params (EchoSenseValue :type Float%20%28single-precision%29))
  (Default|SaveAttributesProgress (CallFunction|GetBoxegameInstance) 3 EchoSenseValue)
  (Default|UpdateEchoSenseAttribute (Variables|Default|Get%20WB%20Character%20Attributes%20Ref))
  (Variables|/Game/_Project/Blueprints/VRPawn.VRPawn_C|SetNumHits (Variables|Default|GetOwnerRef) 0.0))

(fn ResetValues
  (Variables|/Game/_Project/Blueprints/BP_DroneBot.BP_DroneBot_C|SetCanSummonTargets? (Variables|/Game/_Project/Blueprints/VRPawn.VRPawn_C|GetDroneBotRef (Variables|Default|GetOwnerRef)) true)
  (Variables|Timer|SetQuantPunchSessions 1)
  (Variables|Default|SetTimerCurrentValue 0)
  (Variables|Default|SetScoreValue 0)
  (Variables|Default|SetScoreAbsolut 0)
  (bind _widgetref (Variables|Default|GetWidgetRef)
    (:then
      (Variables|/Game/_Project/UI/WI_PlayerHUD.WI_PlayerHUD_C|SetCountRing _widgetref 0)
      (Variables|/Game/_Project/UI/WI_PlayerHUD.WI_PlayerHUD_C|SetCountReload (Variables|Default|GetWidgetRef) 0)
      (Variables|/Game/_Project/UI/WI_PlayerHUD.WI_PlayerHUD_C|SetCountReady (Variables|Default|GetWidgetRef) 0)
      (Variables|/Game/_Project/UI/WI_PlayerHUD.WI_PlayerHUD_C|SetCountUnLoadingBar (Variables|Default|GetWidgetRef) 40)
      (Variables|/Game/_Project/UI/WI_PlayerHUD.WI_PlayerHUD_C|SetCountLoadingBar (Variables|Default|GetWidgetRef) 0)
      (Default|SetPunchValue (Variables|Default|GetWidgetRef))
      (Variables|Default|SetIsSecondTimerPunch false))
    (:else)))

(fn ChangeRoundVariables
  (params (QuantSessions :type Integer) (MaxTimerPunch :type Integer) (MaxTimerRest :type Integer) (DelayUnloadBarTimer :type Float%20%28single-precision%29) (DelayUnloadPBPunchTime :type Float%20%28single-precision%29) (DelayToLoadingBarTimer :type Float%20%28single-precision%29) (DelayLoadingPBPunchTime :type Float%20%28single-precision%29))
  (bind _widgetref (Variables|Default|GetWidgetRef))
  (Variables|Timer|SetQuantSessionsInOneRound QuantSessions)
  (Variables|Timer|SetMaxTimerPunch MaxTimerPunch)
  (Variables|Timer|SetMaxTimerRest MaxTimerRest)
  (Variables|/Game/_Project/UI/WI_PlayerHUD.WI_PlayerHUD_C|SetPercentIncrement _widgetref DelayUnloadPBPunchTime)
  (Variables|/Game/_Project/UI/WI_PlayerHUD.WI_PlayerHUD_C|SetDelayToUnloadBarTimer _widgetref DelayUnloadBarTimer)
  (Variables|Default|SetDelayPBPunchTime DelayLoadingPBPunchTime)
  (Variables|Default|SetDelayLoadingBarTimer DelayToLoadingBarTimer)
  (Variables|Default|SetInitial%20Start%20Delay (Math|Conversions|ToFloat(Integer) (- (Variables|Timer|GetMaxTimerPunch) 2)))
  (CallFunction|ResetValues))

(fn ChargeMana
  (params (ManaByHit :type Float%20%28single-precision%29))
  (Default|IncreaseProgressBarMana (Variables|Default|GetWidgetRef) ManaByHit))

(fn ReturnManatoCharge
  (return (* (+ (* (/ (Math|Conversions|ToFloat(Integer) (Utilities|Struct|BreakS_PlayerInfo (Variables|/Game/_Project/Blueprints/BP_SaveGame.BP_SaveGame_C|GetS_PlayerInfo (Variables|/Game/_Project/Framework/BP_GameInstance.BP_GameInstance_C|GetSaveGame (CallFunction|GetBoxegameInstance))))) 1e+02) 0.2) (Variables|Default|GetBaseMana)) (Variables|Default|GetBoosterToMana))))

(fn DischargeMana
  (params (ManaToDischarge :type Float%20%28single-precision%29))
  (Default|DecreaseProgressBarMana (Variables|Default|GetWidgetRef) ManaToDischarge))

(fn MakeManaBooster1
  (params (BoosterValue :type Float%20%28single-precision%29))
  (Variables|Default|SetBoosterToMana (+ (Variables|Default|GetBoosterToMana) (/ BoosterValue 1e+02))))