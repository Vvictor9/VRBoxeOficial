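; BP_WarningInBattle is a warning actor that makes its SMWarning component blink in and out of view, presumably during battle.
; BeginPlay starts two independent looping timers, one hiding the component and a slightly slower one showing it.
; Because the periods differ, the hidden and visible spans drift over time instead of forming a steady blink.
; Destroyed clears both timer handles.
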(event Custom|WarninigAppear
  (Development|SetHiddeninGame (Variables|Default|GetSM_Warning) false false))

(event Custom|WarningDisappear
  (Development|SetHiddeninGame (Variables|Default|GetSM_Warning) true false))

(event EventBeginPlay
  (bind _returnvalue (Utilities|Time|SetTimerbyEvent (delegate Custom|WarningDisappear) 4.0 true))
  (Variables|Default|SetTH_Disappear _returnvalue)
  (bind _returnvalue_2 (Utilities|Time|SetTimerbyEvent (delegate Custom|WarninigAppear) 4.5 true))
  (Variables|Default|SetTH_Appear _returnvalue_2))

(event Collision|EventActorBeginOverlap
  (params (OtherActor :type Actor%20Object%20Reference)))

(event EventTick
  (params (DeltaSeconds :type Float%20%28single-precision%29)))

(event EventDestroyed
  (Utilities|Time|ClearandInvalidateTimerbyHandle (Variables|Default|GetTH_Appear))
  (Utilities|Time|ClearandInvalidateTimerbyHandle (Variables|Default|GetTH_Disappear)))

(fn ConstructionScript)