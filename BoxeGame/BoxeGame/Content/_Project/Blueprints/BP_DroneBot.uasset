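; Drone sparring opponent for a VR boxing game that faces the player and reacts to glove punches with impulse, sound and sparks.
; Sessions move it into the ring, swap anim instances and start random strafing; stopping retreats it.
; Randomized timers chain attacks: nut projectiles, diversion energy orbs and a melee hit that docks score unless ten punches land in time.
; The game instance's IsPlacebo flag suppresses attacks.
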(event OnComponentEndOverlap(Overlap)
  (params (OverlappedComponent :type Primitive%20Component%20Object%20Reference) (OtherActor :type Actor%20Object%20Reference) (OtherComp :type Primitive%20Component%20Object%20Reference) (OtherBodyIndex :type Integer))
  (if (Utilities|Enum|Equal(Enum) (Utilities|GetObjectName (stale OnComponentBeginOverlap(Overlap) OtherComp)) "SC_GloveR")
    (Utilities|FlowControl|DoOnce false) ; enters at Reset
    (elif (Utilities|Enum|Equal(Enum) (Utilities|GetObjectName (stale OnComponentBeginOverlap(Overlap) OtherComp)) "SC_GloveL")
      (Utilities|FlowControl|DoOnce false) ; enters at Reset
    )))

(event OnComponentEndOverlap(DroneOverlap)
  (params (OverlappedComponent :type Primitive%20Component%20Object%20Reference) (OtherActor :type Actor%20Object%20Reference) (OtherComp :type Primitive%20Component%20Object%20Reference) (OtherBodyIndex :type Integer))
  (bind _returnvalue (Utilities|GetObjectName OtherComp))
  (if (Utilities|Enum|Equal(Enum) _returnvalue "SC_GloveR")
    (Variables|Default|SetFlagRDontEndOverlapYet false)
    (elif (Utilities|Enum|Equal(Enum) _returnvalue "SC_GloveL")
      (Variables|Default|SetFlagLDontEndOverlapYet false))))

(event OnComponentBeginOverlap(Overlap)
  (params (OverlappedComponent :type Primitive%20Component%20Object%20Reference) (OtherActor :type Actor%20Object%20Reference) (OtherComp :type Primitive%20Component%20Object%20Reference) (OtherBodyIndex :type Integer) (bFromSweep :type Boolean) (SweepResult :type Hit%20Result%20Structure%20%28by%20ref%29))
  (bind _returnvalue (Utilities|GetObjectName OtherComp))
  (bind _returnvalue_2 (Transformation|GetWorldLocation OtherComp))
  (bind _droneoverlap (Variables|Default|GetDroneOverlap))
  (bind _returnvalue_3 (Transformation|GetWorldLocation _droneoverlap))
  (bind _returnvalue_4 (- _returnvalue_3 _returnvalue_2))
  (bind _returnvalue_5 (Math|Vector|Normalize _returnvalue_4))
  (bind _returnvalue_6 (* _returnvalue_5 15.0))
  (bind _returnvalue_7 (+ _returnvalue_2 _returnvalue_6))
  (if (Utilities|Enum|Equal(Enum) _returnvalue "SC_GloveR")
    (if (not (Variables|Default|GetFlagRDontEndOverlapYet))
      (Utilities|FlowControl|DoOnce false
        (:Completed
          (Variables|Default|SetFlagRDontEndOverlapYet true)
          (Default|CallOnPunchBag true)
          (Physics|AddImpulseatLocation (Variables|Default|GetSkeletalMesh) (* (* (Math|Vector|GetForwardVector (Variables|Default|GetSkeletalMesh)) -1.0) 1e+03) (.Location (Collision|BreakHitResult SweepResult)) "DronBot" :!label _label)
          (Audio|PlaySoundatLocation "/Game/_Project/Sounds/GameplaySounds/MetalSound_Cue.MetalSound_Cue" (Transformation|GetWorldLocation OtherComp) "0, 0, 0" 0.7 1.0 0.0 0 0 0)
          (Niagara|SpawnSystematLocation "/Game/_Project/NiagaraAbstractSpace3/Effects/NS_Sphere_of_Fireworks.NS_Sphere_of_Fireworks" (Math|Vector|MakeVector (.x _returnvalue_7) (.y _returnvalue_7) (.z (Transformation|GetWorldLocation OtherComp)))))))
    (elif (Utilities|Enum|Equal(Enum) _returnvalue "SC_GloveL")
      (if (not (Variables|Default|GetFlagLDontEndOverlapYet))
        (Utilities|FlowControl|DoOnce false
          (:Completed
            (Variables|Default|SetFlagLDontEndOverlapYet true)
            (Default|CallOnPunchBag false)
            (goto _label)))))))

(event Custom|AiMovement
  (params (HorarioCycle :type Boolean))
  (bind _returnvalue (not HorarioCycle))
  (bind _anim_bp_drone (Variables|Default|GetAnim%20BP%20Drone))
  ;[1 1 1] Movement
  (Utilities|IsValid _anim_bp_drone
    (:Is%20Valid
      (Variables|/Game/_Project/Meshs/AnimBP_Drone.AnimBP_Drone_C|SetCurrentDirection _anim_bp_drone (select HorarioCycle "NewEnumerator2" "NewEnumerator1"))
      (if (Variables|Config|GetCanMove)
        (AI|AIMoveTo self (+ (Transformation|GetActorLocation) (* (Transformation|GetActorRightVector) (select HorarioCycle 5e+01 -5e+01))) 0 1.0 false
          (:OnSuccess
            (if (>= (Math|Random|RandomFloat) 0.8)
              (Variables|/Game/_Project/Meshs/AnimBP_Drone.AnimBP_Drone_C|SetCurrentDirection (Variables|Default|GetAnim%20BP%20Drone) "NewEnumerator0")
              (Utilities|FlowControl|Delay (Math|Random|RandomFloatinRange 2.0 7.0)))
            (CallFunction|AiMovement (select (>= (Math|Random|RandomFloat) 0.3) HorarioCycle _returnvalue)))
          (:OnFail
            (CallFunction|AiMovement _returnvalue)))))))

(event Custom|FireProjectile
  (bind _returnvalue (Math|Random|RandomFloatinRange 0.0 3.0))
  (bind _self self)
  (bind _self_2 self)
  (bind _skeletalmesh (Variables|Default|GetSkeletalMesh))
  (bind _skeletalmesh_2 (Variables|Default|GetSkeletalMesh))
  (bind _returnvalue_2 (Transformation|GetSocketLocation _skeletalmesh "projectileSocket2"))
  (bind _returnvalue_3 (Transformation|GetSocketLocation _skeletalmesh_2 "projectileSocket"))
  ;[1 1 1] Fire projectile
  (if (not (Variables|/Game/_Project/Framework/BP_GameInstance.BP_GameInstance_C|GetIsPlacebo (CallFunction|GetBoxegameInstance)))
    (Components|Movement|StopMovementImmediately (Variables|Character|GetCharacterMovement))
    (Utilities|FlowControl|Delay 0.5)
    (Animation|Montage|PlayMontage (Variables|Default|GetSkeletalMesh) "/Game/_Project/Animations/FireMontage.FireMontage"
      (:then
        (bind _asvrpawn (Utilities|Casting|CastToVRPawn (Game|Player|GetPlayerPawn 0)))
        (Utilities|FlowControl|Sequence
          (:then_0
            (bind _returnvalue_4 (Game|SpawnActorfromClass "/Game/_Project/Blueprints/BP_NutProjectile.BP_NutProjectile_C" (Math|Transform|MakeTransform _returnvalue_3 (Math|Rotator|FindLookatRotation _returnvalue_3 (Transformation|GetWorldLocation (Variables|/Game/_Project/Blueprints/VRPawn.VRPawn_C|GetCamera _asvrpawn))) "1,1,1") "Undefined" _self _self))
            (bind _output_get (Variables|Default|SetCurrentNutProjectileR _returnvalue_4))
            (Transformation|AttachComponentToComponent _output_get (Variables|Default|GetSkeletalMesh) "projectileSocket" "SnapToTarget" "KeepWorld" "KeepWorld" true)
            (Components|Activation|SetActive (Variables|Default|GetNiagara) true true))
          (:then_1
            (bind _returnvalue_5 (Game|SpawnActorfromClass "/Game/_Project/Blueprints/BP_NutProjectile.BP_NutProjectile_C" (Math|Transform|MakeTransform _returnvalue_2 (Math|Rotator|FindLookatRotation _returnvalue_2 (Transformation|GetWorldLocation (Variables|/Game/_Project/Blueprints/VRPawn.VRPawn_C|GetCamera _asvrpawn))) "1,1,1") "Undefined" _self_2 _self_2))
            (bind _output_get_2 (Variables|Default|SetCurrentNutProjectileL _returnvalue_5))
            (Transformation|AttachComponentToComponent _output_get_2 (Variables|Default|GetSkeletalMesh) "projectileSocket2" "SnapToTarget" "KeepWorld" "KeepWorld" true))
          (:then_2
            (Utilities|FlowControl|Delay 2.0)
            (Components|Activation|SetActive (Variables|Default|GetNiagara) false true)
            (Utilities|FlowControl|Sequence
              (:then_0
                (Utilities|FlowControl|Delay _returnvalue)
                (bind _currentnutprojectiler (Variables|Default|GetCurrentNutProjectileR)
                  (:then
                    (Transformation|DetachFromActor _currentnutprojectiler "KeepWorld" "KeepWorld" "KeepWorld")
                    (Default|Shot _currentnutprojectiler))
                  (:else)))
              (:then_1
                (Utilities|FlowControl|Delay _returnvalue)
                (bind _currentnutprojectilel (Variables|Default|GetCurrentNutProjectileL)
                  (:then
                    (Transformation|DetachFromActor _currentnutprojectilel "KeepWorld" "KeepWorld" "KeepWorld")
                    (Default|Shot _currentnutprojectilel))
                  (:else)))))))
      (:OnCompleted
        ;;[1 1 1] On complete montage
        (CallFunction|AiMovement (Math|Random|RandomBool))
        (if (Variables|Default|GetCanFire)
          (switch int (Math|Random|RandomIntegerinRange 0 2)
            (:0
              (bind _returnvalue_6 (Utilities|Time|SetTimerbyEvent (EventDispatchers|CreateEvent :!event Custom|FireProjectile) (Math|Random|RandomFloatinRange 2.0 4.0)))
              (Variables|Default|SetLoopSpawnProjectiles _returnvalue_6))
            (:1
              (bind _returnvalue_7 (Utilities|Time|SetTimerbyEvent (EventDispatchers|CreateEvent :!event Custom|FireDiversionProjectile) (Math|Random|RandomFloatinRange 2.0 4.0)))
              (Variables|Default|SetLoopSpawnProjectiles _returnvalue_7))
            (:2
              (bind _returnvalue_8 (Utilities|Time|SetTimerbyEvent (EventDispatchers|CreateEvent :!event Custom|MeeleHit) (Math|Random|RandomFloatinRange 1.0 2.0)))
              (Variables|Default|SetLoopSpawnProjectiles _returnvalue_8))))))))

(event Custom|ChangeDroneCondition
  (params (Condition :type EN_Condition%20Enum :default "NewEnumerator0"))
  (Variables|/Game/_Project/Meshs/AnimBP_DroneRestTime.AnimBP_DroneRestTime_C|SetCondition (Variables|Default|GetAnim%20BP%20Drone%20Rest%20Time) Condition))

(event Custom|AiMoveOutOfRing
  (bind _vrpawnref (Variables|Default|GetVRPawnRef))
  (bind _returnvalue (Transformation|GetActorLocation _vrpawnref))
  ;[1 1 1] Move Drone To ring
  (Physics|SetSimulatePhysics (Variables|Default|GetSkeletalMesh) false)
  (Components|Movement|StopMovementImmediately (Variables|Character|GetCharacterMovement))
  (Variables|/Game/_Project/Meshs/AnimBP_DroneRestTime.AnimBP_DroneRestTime_C|SetCondition (Variables|Default|GetAnim%20BP%20Drone%20Rest%20Time) "NewEnumerator3")
  (AI|AIMoveTo (AI|GetAIController (Pawn|GetController)) (+ (Math|Vector|MakeVector (.x _returnvalue) (.y _returnvalue) 8e+01) (* (Transformation|GetActorForwardVector _vrpawnref) 6.5e+02)) 0 1.0 "Default" "Default" true true
    (:OnRequestFailed
      (CallFunction|AiMoveOutOfRing))))

(event Custom|DroneHeightAdjustments
  (bind _skeletalmesh (Variables|Default|GetSkeletalMesh))
  (bind _returnvalue (Transformation|GetWorldLocation _skeletalmesh))
  (Variables|Default|SetZLocationToAdjust (- (.z (Transformation|GetWorldLocation (Variables|Default|GetSkeletalMesh))) 1e+02))
  (bind _newtrack_1 (Timeline|THAdjustHeight PlayFromStart)
    (:Update
      (Transformation|SetWorldLocation (Variables|Default|GetSkeletalMesh) (Math|Vector|Lerp(Vector) (Transformation|GetWorldLocation _skeletalmesh) (Math|Vector|MakeVector (.x _returnvalue) (.y _returnvalue) (Variables|Default|GetZLocationToAdjust)) _newtrack_1) false false))))

(event Custom|OnStartSession
  ;[1 1 1] Active projetiles loop
  (Utilities|FlowControl|Sequence
    (:then_0
      (Utilities|FlowControl|Delay 2.0)
      (CallFunction|ChangeDroneCondition "NewEnumerator2")
      (CallFunction|AiMovetoRingue))
    (:then_1
      (Utilities|FlowControl|Delay 4.0)
      (CallFunction|ChangeAnimInstance "/Game/_Project/Meshs/AnimBP_Drone.AnimBP_Drone_C")
      (Class|NavModifierComponent|SetAreaClass (Variables|/Game/_Project/Blueprints/BP_NavMod.BP_NavMod_C|GetNavModifier (Variables|Default|GetNavModRef)) "/Script/NavigationSystem.NavArea_Null")
      (Physics|SetSimulatePhysics (Variables|Default|GetSkeletalMesh) true)
      (Utilities|FlowControl|Delay 2.0)
      (CallFunction|AiMovement (Math|Random|RandomBool)))
    (:then_2
      (Utilities|FlowControl|Delay 6.0)
      (switch int (Math|Random|RandomIntegerinRange 0 0)
        (:0
          (bind _returnvalue (Utilities|Time|SetTimerbyEvent (EventDispatchers|CreateEvent :!event Custom|FireProjectile) (Math|Random|RandomFloatinRange 2.0 4.0)))
          (Variables|Default|SetLoopSpawnProjectiles _returnvalue))
        (:1
          (bind _returnvalue_2 (Utilities|Time|SetTimerbyEvent (EventDispatchers|CreateEvent :!event Custom|FireDiversionProjectile) (Math|Random|RandomFloatinRange 2.0 4.0)))
          (Variables|Default|SetLoopSpawnProjectiles _returnvalue_2))
        (:2
          (bind _returnvalue_3 (Utilities|Time|SetTimerbyEvent (EventDispatchers|CreateEvent :!event Custom|MeeleHit) (Math|Random|RandomFloatinRange 1.0 2.0)))
          (Variables|Default|SetLoopSpawnProjectiles _returnvalue_3)))
      (Variables|Default|SetCanFire true))))

(event Custom|OnStopSession
  ;[1 1 1] Active projetiles loop
  (Utilities|FlowControl|Sequence
    (:then_0
      (CallFunction|DestroyEnergyOrb)
      (Utilities|Time|ClearandInvalidateTimerbyHandle (Variables|Default|GetLoopSpawnProjectiles))
      (Variables|Default|SetCanFire false))
    (:then_1
      (CallFunction|ChangeAnimInstance "/Game/_Project/Meshs/AnimBP_DroneRestTime.AnimBP_DroneRestTime_C"))
    (:then_2
      (Utilities|FlowControl|Delay 2.0)
      (CallFunction|AiMoveOutOfRing))))

(event Custom|StopRound
  (params (ScoreValue :type Integer) (ScoreAbsolut :type Integer))
  (CallFunction|OnStopSession))

(event Custom|MeeleHit
  ;[1 1 1] MeeleAtack
  (Variables|/Game/_Project/Meshs/AnimBP_Drone.AnimBP_Drone_C|SetLoop%20Animation (Variables|Default|GetAnim%20BP%20Drone) true)
  (Variables|/Game/_Project/Meshs/AnimBP_Drone.AnimBP_Drone_C|SetCurrentHit (Variables|Default|GetAnim%20BP%20Drone) "NewEnumerator0")
  (if (not (Variables|/Game/_Project/Framework/BP_GameInstance.BP_GameInstance_C|GetIsPlacebo (CallFunction|GetBoxegameInstance)))
    (Components|Movement|StopMovementImmediately (Variables|Character|GetCharacterMovement))
    (Variables|Config|SetCanMove false)
    (Variables|/Game/_Project/Meshs/AnimBP_Drone.AnimBP_Drone_C|SetLoop%20Animation (Variables|Default|GetAnim%20BP%20Drone) false)
    (Utilities|FlowControl|Delay 0.5)
    (AI|AIMoveTo self "0, 0, 0" (Game|Player|GetPlayerPawn 0) 2e+01 true
      (:OnSuccess
        (Animation|Montage|PlayMontage (Variables|Default|GetSkeletalMesh) "/Game/_Project/Animations/PrepareHitMontage.PrepareHitMontage" 0.5
          (:OnCompleted
            (bind _asvrpawn (Utilities|Casting|CastToVRPawn (Game|Player|GetPlayerPawn 0)))
            (Utilities|FlowControl|Sequence
              (:then_0
                (Variables|/Game/_Project/Blueprints/VRPawn.VRPawn_C|SetNumPunchs _asvrpawn 0)
                (EventDispatchers|BindEventtoOnSubtractScore (EventDispatchers|CreateEvent :!event Custom|SubtractScoreByHit)))
              (:then_1
                (bind _returnvalue (Utilities|Time|SetTimerbyEvent (delegate Custom|ResetNumPunchs) 0.1 true))
                (Variables|Default|SetTimerToResetNumPunchs _returnvalue))
              (:then_2
                (Utilities|FlowControl|Delay 3.0)
                (Utilities|Time|ClearandInvalidateTimerbyHandle (Variables|Default|GetTimerToResetNumPunchs))
                (Default|CallOnSubtractScore))
              (:then_3
                ;;[1 1 1] On Complete PlayMontage
                (Utilities|FlowControl|Delay 4.0)
                (Variables|/Game/_Project/Meshs/AnimBP_Drone.AnimBP_Drone_C|SetCurrentHit (Variables|Default|GetAnim%20BP%20Drone) "NewEnumerator2")
                (Variables|Config|SetCanMove true)
                (CallFunction|AiMovement (Math|Random|RandomBool))
                (if (Variables|Default|GetCanFire)
                  (switch int (Math|Random|RandomIntegerinRange 0 2)
                    (:0
                      (bind _returnvalue_2 (Utilities|Time|SetTimerbyEvent (EventDispatchers|CreateEvent :!event Custom|FireProjectile) (Math|Random|RandomFloatinRange 2.0 4.0)))
                      (Variables|Default|SetLoopSpawnProjectiles _returnvalue_2))
                    (:1
                      (bind _returnvalue_3 (Utilities|Time|SetTimerbyEvent (EventDispatchers|CreateEvent :!event Custom|FireDiversionProjectile) (Math|Random|RandomFloatinRange 2.0 4.0)))
                      (Variables|Default|SetLoopSpawnProjectiles _returnvalue_3))
                    (:2
                      (bind _returnvalue_4 (Utilities|Time|SetTimerbyEvent (EventDispatchers|CreateEvent :!event Custom|MeeleHit) (Math|Random|RandomFloatinRange 1.0 2.0)))
                      (Variables|Default|SetLoopSpawnProjectiles _returnvalue_4))))))))))))

(event Custom|ResetNumPunchs
  ;[1 1 1] MeeleAtack
  (if (== (Variables|/Game/_Project/Blueprints/VRPawn.VRPawn_C|GetNumPunchs (stale Custom|MeeleHit _asvrpawn)) 10)
    (bind _asvrpawn (Utilities|Casting|CastToVRPawn (Game|Player|GetPlayerPawn 0)))
    (Variables|/Game/_Project/Blueprints/VRPawn.VRPawn_C|SetNumPunchs _asvrpawn 0)
    (Utilities|Time|ClearandInvalidateTimerbyHandle (Variables|Default|GetTimerToResetNumPunchs))
    (EventDispatchers|UnbindallEventsfromOnSubtractScore)))

(event Custom|SubtractScoreByHit
  (bind _anim_bp_drone (Variables|Default|GetAnim%20BP%20Drone))
  ;[1 1 1] Play AnimMontage to Subtract Score
  (Utilities|IsValid _anim_bp_drone
    (:Is%20Valid
      (Variables|/Game/_Project/Meshs/AnimBP_Drone.AnimBP_Drone_C|SetCurrentHit _anim_bp_drone "NewEnumerator1")
      (Animation|Montage|PlayMontage 0 "/Game/_Project/Animations/Anim_DroneBot_Hit4_Montage.Anim_DroneBot_Hit4_Montage" 0.5
        (:OnCompleted
          (Variables|/Game/_Project/Meshs/AnimBP_Drone.AnimBP_Drone_C|SetLoop%20Animation (Variables|Default|GetAnim%20BP%20Drone) false)
          (bind _asvrpawn (Utilities|Casting|CastToVRPawn (Game|Player|GetPlayerPawn 0)))
          (Default|AddPunchValue (Variables|/Game/_Project/Blueprints/VRPawn.VRPawn_C|GetBPC_Timer _asvrpawn) (Math|Conversions|ToFloat(Integer) (* (/ (Variables|/Game/_Project/Blueprints/Component/BPC_RoundController.BPC_RoundController_C|GetScoreValue (Variables|/Game/_Project/Blueprints/VRPawn.VRPawn_C|GetBPC_Timer _asvrpawn)) 5) -1)) 0.0)
          (Variables|/Game/_Project/Blueprints/VRPawn.VRPawn_C|SetNumPunchs _asvrpawn 0)
          (Utilities|Time|ClearandInvalidateTimerbyHandle (Variables|Default|GetTimerToResetNumPunchs)))))))

(event Custom|FireDiversionProjectile
  (bind _returnvalue (Math|Random|RandomFloatinRange 0.0 3.0))
  (bind _self self)
  (bind _self_2 self)
  (bind _skeletalmesh (Variables|Default|GetSkeletalMesh))
  (bind _skeletalmesh_2 (Variables|Default|GetSkeletalMesh))
  (bind _returnvalue_2 (Transformation|GetSocketLocation _skeletalmesh "projectileSocket2"))
  (bind _returnvalue_3 (Transformation|GetSocketLocation _skeletalmesh_2 "projectileSocket"))
  ;[1 1 1] Fire Diversion Projectile
  (if (not (Variables|/Game/_Project/Framework/BP_GameInstance.BP_GameInstance_C|GetIsPlacebo (CallFunction|GetBoxegameInstance)))
    (Components|Movement|StopMovementImmediately (Variables|Character|GetCharacterMovement))
    (Utilities|FlowControl|Delay 0.5)
    (Animation|Montage|PlayMontage (Variables|Default|GetSkeletalMesh) "/Game/_Project/Animations/FireMontage.FireMontage"
      (:then
        (bind _asvrpawn (Utilities|Casting|CastToVRPawn (Game|Player|GetPlayerPawn 0)))
        (Utilities|FlowControl|Sequence
          (:then_0
            (bind _returnvalue_4 (Game|SpawnActorfromClass "/Game/_Project/Blueprints/EnergyOrb/BP_EnergyOrb.BP_EnergyOrb_C" (Math|Transform|MakeTransform _returnvalue_3 (Math|Rotator|FindLookatRotation _returnvalue_3 (Transformation|GetWorldLocation (Variables|/Game/_Project/Blueprints/VRPawn.VRPawn_C|GetCamera _asvrpawn))) "1,1,1") "Undefined" _self_2 _self_2))
            (bind _output_get (Variables|Default|SetCurrentDiversionProjectileR _returnvalue_4))
            (Transformation|AttachComponentToComponent _output_get (Variables|Default|GetSkeletalMesh) "projectileSocket" "SnapToTarget" "KeepWorld" "KeepWorld" true)
            (Components|Activation|SetActive (Variables|Default|GetNiagara) true true))
          (:then_1
            (bind _returnvalue_5 (Game|SpawnActorfromClass "/Game/_Project/Blueprints/EnergyOrb/BP_EnergyOrb.BP_EnergyOrb_C" (Math|Transform|MakeTransform _returnvalue_2 (Math|Rotator|FindLookatRotation _returnvalue_2 (Transformation|GetWorldLocation (Variables|/Game/_Project/Blueprints/VRPawn.VRPawn_C|GetCamera _asvrpawn))) "1,1,1") "Undefined" _self _self))
            (bind _output_get_2 (Variables|Default|SetCurrentDiversionProjectileL _returnvalue_5))
            (Transformation|AttachComponentToComponent _output_get_2 (Variables|Default|GetSkeletalMesh) "projectileSocket2" "SnapToTarget" "KeepWorld" "KeepWorld" true))
          (:then_2
            (Utilities|FlowControl|Delay 2.0)
            (Components|Activation|SetActive (Variables|Default|GetNiagara) false true)
            (Utilities|FlowControl|Sequence
              (:then_0
                (Utilities|FlowControl|Delay _returnvalue)
                (bind _currentdiversionprojectiler (Variables|Default|GetCurrentDiversionProjectileR)
                  (:then
                    (Transformation|DetachFromActor _currentdiversionprojectiler "KeepWorld" "KeepWorld" "KeepWorld"))
                  (:else)))
              (:then_1
                (Utilities|FlowControl|Delay _returnvalue)
                (bind _currentdiversionprojectilel (Variables|Default|GetCurrentDiversionProjectileL)
                  (:then
                    (Transformation|DetachFromActor _currentdiversionprojectilel "KeepWorld" "KeepWorld" "KeepWorld"))
                  (:else)))))))
      (:OnCompleted
        ;;[1 1 1] On complete montage
        (CallFunction|AiMovement (Math|Random|RandomBool))
        (if (Variables|Default|GetCanFire)
          (switch int (Math|Random|RandomIntegerinRange 0 2)
            (:0
              (bind _returnvalue_6 (Utilities|Time|SetTimerbyEvent (EventDispatchers|CreateEvent :!event Custom|FireProjectile) (Math|Random|RandomFloatinRange 2.0 4.0)))
              (Variables|Default|SetLoopSpawnProjectiles _returnvalue_6))
            (:1
              (bind _returnvalue_7 (Utilities|Time|SetTimerbyEvent (EventDispatchers|CreateEvent :!event Custom|FireDiversionProjectile) (Math|Random|RandomFloatinRange 2.0 4.0)))
              (Variables|Default|SetLoopSpawnProjectiles _returnvalue_7))
            (:2
              (bind _returnvalue_8 (Utilities|Time|SetTimerbyEvent (EventDispatchers|CreateEvent :!event Custom|MeeleHit) (Math|Random|RandomFloatinRange 1.0 2.0)))
              (Variables|Default|SetLoopSpawnProjectiles _returnvalue_8)))
          (CallFunction|DestroyEnergyOrb))))))

(event Custom|AiMoveToRingue
  (bind _vrpawnref (Variables|Default|GetVRPawnRef))
  (bind _returnvalue (Transformation|GetActorLocation _vrpawnref))
  ;[1 1 1] Move Drone To ring
  (Physics|SetSimulatePhysics (Variables|Default|GetSkeletalMesh) false)
  (Components|Movement|StopMovementImmediately (Variables|Character|GetCharacterMovement))
  (Variables|/Game/_Project/Meshs/AnimBP_DroneRestTime.AnimBP_DroneRestTime_C|SetCondition (Variables|Default|GetAnim%20BP%20Drone%20Rest%20Time) "NewEnumerator3")
  (AI|AIMoveTo (AI|GetAIController (Pawn|GetController)) (+ (Math|Vector|MakeVector (.x _returnvalue) (.y _returnvalue) 8e+01) (* (Transformation|GetActorForwardVector _vrpawnref) 8e+01)) 0 1.0 "Default" "Default" true true
    (:OnRequestFailed
      (CallFunction|AiMovetoRingue))))

(event EventBeginPlay
  (bind _asvrpawn (Utilities|Casting|CastToVRPawn (Game|Player|GetPlayerPawn 0)))
  (Variables|Default|SetVRPawnRef _asvrpawn)
  (Utilities|FlowControl|Delay 2.0)
  (bind _asanim_bp_drone_rest_time (Utilities|Casting|CastToAnimBP_DroneRestTime (Components|SkeletalMesh|GetAnimInstance (Variables|Default|GetSkeletalMesh))))
  (bind _output_get (Variables|Default|SetAnim%20BP%20Drone%20Rest%20Time _asanim_bp_drone_rest_time))
  (Variables|/Game/_Project/Meshs/AnimBP_DroneRestTime.AnimBP_DroneRestTime_C|SetCondition _output_get "NewEnumerator0")
  (Pawn|Components|CharacterMovement|SetMovementMode (Variables|Character|GetCharacterMovement) "MOVE_Flying" 0)
  (bind _outactors (Actor|GetAllActorsOfClass "/Game/_Project/Blueprints/BP_NavMod.BP_NavMod_C"))
  (Variables|Default|SetNavModRef (Utilities|Array|Get(acopy) _outactors))
  (bind _asvrpawn_2 (Utilities|Casting|CastToVRPawn (Game|Player|GetPlayerPawn 0)))
  (EventDispatchers|BindEventtoStartPunchTime (Variables|/Game/_Project/Blueprints/VRPawn.VRPawn_C|GetBPC_Timer _asvrpawn_2) (EventDispatchers|CreateEvent :!event Custom|OnStartSession))
  (EventDispatchers|BindEventtoStartRestTime (Variables|/Game/_Project/Blueprints/VRPawn.VRPawn_C|GetBPC_Timer _asvrpawn_2) (EventDispatchers|CreateEvent :!event Custom|OnStopSession))
  (EventDispatchers|BindEventtoOnEndRound (CallFunction|GetBoxegameInstance) (delegate Custom|StopRound))
  (EventDispatchers|BindEventtoOnSubtractScore (EventDispatchers|CreateEvent :!event Custom|SubtractScoreByHit)))

(event EventTick
  (params (DeltaSeconds :type Float%20%28single-precision%29))
  (Transformation|SetActorRotation (Math|Rotator|MakeRotator 0.0 0.0 (.yaw (Math|Rotator|FindLookatRotation (Transformation|GetActorLocation) (Transformation|GetActorLocation (Pawn|GetControlledPawn (Game|GetPlayerController 0))))))))

(fn ConstructionScript)

(fn DestroyEnergyOrb
  (bind _currentdiversionprojectiler (Variables|Default|GetCurrentDiversionProjectileR))
  (bind _currentdiversionprojectilel (Variables|Default|GetCurrentDiversionProjectileL))
  (Utilities|IsValid _currentdiversionprojectiler
    (:Is%20Valid
      (Actor|DestroyActor _currentdiversionprojectiler)
      (Utilities|IsValid _currentdiversionprojectilel
        (:Is%20Valid
          (Actor|DestroyActor _currentdiversionprojectilel))))))

(fn ChangeAnimInstance
  (params (AnimClassRef :type Object%20Class%20Reference))
  (bind _skeletalmesh (Variables|Default|GetSkeletalMesh))
  (bind _returnvalue (Components|SkeletalMesh|GetAnimInstance _skeletalmesh))
  (Class|SkeletalMeshComponent|SetAnimClass (Variables|Default|GetSkeletalMesh) AnimClassRef)
  (Utilities|FlowControl|Sequence
    (:then_0
      (bind _asanim_bp_drone (Utilities|Casting|CastToAnimBP_Drone _returnvalue)
        (:then
          (bind _output_get (Variables|Default|SetAnim%20BP%20Drone _asanim_bp_drone))
          (Variables|/Game/_Project/Meshs/AnimBP_Drone.AnimBP_Drone_C|SetCurrentDirection _output_get "NewEnumerator0"))
        (:CastFailed
          (Variables|Default|SetAnim%20BP%20Drone 0))))
    (:then_1
      (bind _asanim_bp_drone_rest_time (Utilities|Casting|CastToAnimBP_DroneRestTime _returnvalue)
        (:then
          (bind _output_get_2 (Variables|Default|SetAnim%20BP%20Drone%20Rest%20Time _asanim_bp_drone_rest_time))
          (Variables|/Game/_Project/Meshs/AnimBP_DroneRestTime.AnimBP_DroneRestTime_C|SetCondition _output_get_2 "NewEnumerator2"))
        (:CastFailed
          (Variables|Default|SetAnim%20BP%20Drone%20Rest%20Time 0))))))