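; BP_GradeLaser is a moving laser hazard that cuts a tenth of the VR player's score on contact.
; After BeginPlay it briefly waits, then reveals its two laser effects and plays an attached looping-style audio cue.
; MoveGradeLaser waits, yaws toward the VRPawn, and runs a rate-adjustable timeline that pushes it forward, destroying it when finished.
; Overlapping the VRPawn destroys the laser and sends the negative points to the pawn's BPCTimer via AddPunchValue.
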(event OnComponentBeginOverlap(Box)
  (params (OverlappedComponent :type Primitive%20Component%20Object%20Reference) (OtherActor :type Actor%20Object%20Reference) (OtherComp :type Primitive%20Component%20Object%20Reference) (OtherBodyIndex :type Integer) (bFromSweep :type Boolean) (SweepResult :type Hit%20Result%20Structure%20%28by%20ref%29))
  (bind _asvrpawn (Utilities|Casting|CastToVRPawn OtherActor))
  (Actor|DestroyActor)
  (Default|AddPunchValue (Variables|/Game/_Project/Blueprints/VRPawn.VRPawn_C|GetBPC_Timer _asvrpawn) (Math|Conversions|ToFloat(Integer) (* (/ (Variables|/Game/_Project/Blueprints/Component/BPC_RoundController.BPC_RoundController_C|GetScoreValue (Variables|/Game/_Project/Blueprints/VRPawn.VRPawn_C|GetBPC_Timer _asvrpawn)) 10) -1)) 0.0))

(event Custom|MoveGradeLaser
  (params (NewTimeLinePlayRate :type Float%20%28single-precision%29))
  (Utilities|FlowControl|Delay 2.0)
  (bind _asvrpawn (Utilities|Casting|CastToVRPawn (Game|Player|GetPlayerPawn 0)))
  (bind _output_get (Variables|Default|SetVRPawnRef _asvrpawn))
  (Transformation|SetActorRotation (Math|Rotator|MakeRotator 0.0 0.0 (.yaw (Math|Rotator|FindLookatRotation (Transformation|GetActorLocation) (Transformation|GetActorLocation _output_get)))))
  (Components|Timeline|SetPlayRate (Variables|Default|GetTL_MoveGradeLaser) NewTimeLinePlayRate)
  (bind _alpha (Timeline|TL_MoveGradeLaser PlayFromStart)
    (:Update
      (Transformation|SetActorLocation (Math|Vector|Lerp(Vector) (Transformation|GetActorLocation) (+ (Transformation|GetActorLocation) (* (Transformation|GetActorForwardVector) 3.5e+02)) _alpha) false false))
    (:Finished
      (Actor|DestroyActor))))

(event EventBeginPlay
  (Utilities|FlowControl|Delay 0.5)
  (Development|SetHiddeninGame (Variables|Default|GetNS_Laser1) false false)
  (bind _returnvalue (Audio|SpawnSoundAttached "/Game/_Project/Sounds/cues/Futuristic/Interface_Data_Processing_Futuristic_53_Cue.Interface_Data_Processing_Futuristic_53_Cue" (Variables|Default|GetDefaultSceneRoot) "None" "0, 0, 0" "0, 0, 0" "KeepRelativeOffset" true 1.0 1.0 0.0 0 0))
  (Variables|Default|SetLeaserAudioRef _returnvalue))

(fn ConstructionScript)