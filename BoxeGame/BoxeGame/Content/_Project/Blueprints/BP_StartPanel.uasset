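; BP_StartPanel is a VR start panel that begins a new round when the VRPawn overlaps its box and the round-mode check is false.
; Any overlap plays a warning sound and hides the panel, even before the pawn cast.
; HidePanel and ShowPanel toggle visibility and run timelines that nudge the panel and the BP_HUDNewScore found at BeginPlay down or up by fixed per-update offsets.
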(event OnComponentBeginOverlap(Box)
  (params (OverlappedComponent :type Primitive%20Component%20Object%20Reference) (OtherActor :type Actor%20Object%20Reference) (OtherComp :type Primitive%20Component%20Object%20Reference) (OtherBodyIndex :type Integer) (bFromSweep :type Boolean) (SweepResult :type Hit%20Result%20Structure%20%28by%20ref%29))
  (Audio|SpawnSound2D "/Game/_Project/Sounds/HistorySounds/NewSounds/aviso.aviso" 1.0 1.0 0.0 0)
  (CallFunction|HidePanel)
  (bind _asvrpawn (Utilities|Casting|CastToVRPawn OtherActor))
  (if (not (Variables|/Game/_Project/Blueprints/Component/BPC_RoundController.BPC_RoundController_C|GetSetIsInRoundMode? (Variables|/Game/_Project/Blueprints/VRPawn.VRPawn_C|GetBPC_Timer _asvrpawn)))
    (Default|StartNewRound _asvrpawn)))

(event Custom|HidePanel
  (Rendering|SetActorHiddenInGame true)
  (Timeline|TH_HidePanel PlayFromStart
    (:Update
      (Transformation|AddActorLocalOffset "0, 0,-3.000000" false false)
      (Transformation|AddActorLocalOffset (Variables|Default|GetBPHudNewScoreRef) "0, 0,-3.000000" false false))))

(event Custom|ShowPanel
  (Rendering|SetActorHiddenInGame false)
  (Timeline|TH_ShowPanel PlayFromStart
    (:Update
      (Transformation|AddActorLocalOffset "0, 0,3.000000" false false)
      (Transformation|AddActorLocalOffset (Variables|Default|GetBPHudNewScoreRef) "0, 0,3.000000" false false))))

(event EventBeginPlay
  (bind _outactors (Actor|GetAllActorsOfClass "/Game/_Project/Blueprints/BP_HUDNewScore.BP_HUDNewScore_C"))
  (Variables|Default|SetBPHudNewScoreRef (Utilities|Array|Get(acopy) _outactors)))

(fn ConstructionScript)