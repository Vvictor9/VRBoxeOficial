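; Save game Blueprint holding a 20-slot score leaderboard, per-block point history and player attribute progression.
; New scores are inserted after a descending selection sort, trimming the overflow entry; helpers check for records and reset slots to "Empty".
; Block points form a rolling 20-entry list.
; Experience levels the chosen attribute and the player (stored at attribute index 4), discarding surplus EXP on level-up.
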(fn AddNewRankSave
  (params (PlayerName :type Text) (TotalScore :type Integer) (ScoreAbsolut :type Integer))
  (bind _saverankinginfo (Variables|Default|GetSaveRankingInfo))
  (CallFunction|OrganizeArray)
  (bind (_array_element _array_index) (Utilities|Array|ForEachLoopwithBreak (Variables|Default|GetSaveRankingInfo) :!label _label)
    (:LoopBody
      (if (<= (.TotalScoreValue (Utilities|Struct|BreakS_SaveRanking _array_element)) TotalScore)
        (Utilities|Array|Insert _saverankinginfo (Utilities|Struct|MakeS_SaveRanking PlayerName TotalScore (Math|DateTime|Now) ScoreAbsolut) _array_index)
        (Utilities|Array|RemoveIndex _saverankinginfo 20)
        (goto _label Break)))))

(fn ResetSaveValues
  (bind _s_saveranking (Utilities|Struct|MakeS_SaveRanking "Empty" 0 "0001.01.01-00.00.00"))
  (Variables|Default|SetSaveRankingInfo (Utilities|Array|MakeArray _s_saveranking _s_saveranking _s_saveranking _s_saveranking _s_saveranking _s_saveranking _s_saveranking _s_saveranking _s_saveranking _s_saveranking _s_saveranking _s_saveranking _s_saveranking _s_saveranking _s_saveranking _s_saveranking _s_saveranking _s_saveranking _s_saveranking _s_saveranking)))

(fn OrganizeArray
  (bind _saverankinginfo (Variables|Default|GetSaveRankingInfo))
  (for _index (range 0 (- (Utilities|Array|Length (Variables|Default|GetSaveRankingInfo)) 1))
    (LocalVariables|SetCurrentBiggerRankValue (Utilities|Array|Get(acopy) (Variables|Default|GetSaveRankingInfo) _index))
    (LocalVariables|SetCurrentBiggerIndex _index)
    (for _index_2 (range (+ _index 1) (- (Utilities|Array|Length (Variables|Default|GetSaveRankingInfo)) 1))
      (if (>= (.totalscorevalue (Utilities|Array|Get(acopy) (Variables|Default|GetSaveRankingInfo) _index_2)) (.totalscorevalue (LocalVariables|GetCurrentBiggerRankValue)))
        (LocalVariables|SetCurrentBiggerRankValue (Utilities|Array|Get(acopy) (Variables|Default|GetSaveRankingInfo) _index_2))
        (LocalVariables|SetCurrentBiggerIndex _index_2)))
    (LocalVariables|SetAuxValorRankStruct (Utilities|Array|Get(acopy) (Variables|Default|GetSaveRankingInfo) _index))
    (Utilities|Array|SetArrayElem _saverankinginfo _index (LocalVariables|GetCurrentBiggerRankValue))
    (Utilities|Array|SetArrayElem _saverankinginfo (LocalVariables|GetCurrentBiggerIndex) (LocalVariables|GetAuxValorRankStruct))))

(fn IsNewRecord?
  (params (TotalValue :type Integer))
  (for _array_element (Variables|Default|GetSaveRankingInfo)
    (if (<= (.TotalScoreValue (Utilities|Struct|BreakS_SaveRanking _array_element)) TotalValue)
      (return true)))
  (return false))

(fn AddPointstoEachBlock
  (params (PointByRound :type Integer))
  (bind _savepontuacaobloco (Variables|Default|GetSavePontuacaoBloco))
  (bind _savepontuacaobloco_2 (Variables|Default|GetSavePontuacaoBloco))
  (bind _savepontuacaobloco_3 (Variables|Default|GetSavePontuacaoBloco))
  (bind _pontuaçãobloco (Utilities|Struct|BreakS_PontuaçãoBlocos _savepontuacaobloco))
  (bind _pontuaçãobloco_2 (Utilities|Struct|BreakS_PontuaçãoBlocos _savepontuacaobloco_2))
  (bind _pontuaçãobloco_3 (Utilities|Struct|BreakS_PontuaçãoBlocos _savepontuacaobloco_3))
  (if (== (Utilities|Array|Length (Utilities|Struct|BreakS_PontuaçãoBlocos (Variables|Default|GetSavePontuacaoBloco))) 20)
    (Variables|Default|SetlastScoreAdd (Utilities|Array|Get(acopy) _pontuaçãobloco_2 (- (Utilities|Array|Length _pontuaçãobloco_2) 1)))
    (Utilities|Array|RemoveIndex _pontuaçãobloco)
    (Utilities|Array|Add _pontuaçãobloco PointByRound)
    (else
      (Variables|Default|SetlastScoreAdd (Utilities|Array|Get(acopy) _pontuaçãobloco_3 (- (Utilities|Array|Length _pontuaçãobloco_3) 1)))
      (Utilities|Array|Add (Utilities|Struct|BreakS_PontuaçãoBlocos (Variables|Default|GetSavePontuacaoBloco)) PointByRound))))

(fn SetAttributebyIndex
  (params (Index :type Integer) (ExpAttributo :type Float%20%28single-precision%29) (ExpPlayer :type Float%20%28single-precision%29))
  (bind _returnvalue (/ ExpAttributo 1e+02))
  (bind _returnvalue_2 (/ ExpPlayer 1e+02))
  (bind _s_attributos (Variables|Default|GetS_Attributos))
  (bind _s_attributos_2 (Variables|Default|GetS_Attributos))
  (bind _s_attributos_3 (Variables|Default|GetS_Attributos))
  (bind _output (Utilities|Array|Get(acopy) _s_attributos 4))
  (bind _output_2 (Utilities|Array|Get(acopy) _s_attributos_3 Index))
  (bind _output_3 (Utilities|Array|Get(acopy) _s_attributos_2 4))
  (bind (_name _level _exptolevelup _upgrade _expupgrade _playername _playerlevel _playerexp) (Utilities|Struct|BreakS_Attributos _output_2))
  (bind (_name_2 _level_2 _exptolevelup_2 _upgrade_2 _expupgrade_2 _playername_2 _playerlevel_2 _playerexp_2) (Utilities|Struct|BreakS_Attributos _output))
  (bind (_name_3 _level_3 _exptolevelup_3 _upgrade_3 _expupgrade_3 _playername_3 _playerlevel_3) (Utilities|Struct|BreakS_Attributos _output_3))
  (bind _returnvalue_3 (+ _playerexp_2 _returnvalue_2))
  (bind _returnvalue_4 (+ _exptolevelup _returnvalue))
  (Variables|Default|SetIndex Index)
  (if (>= _returnvalue_3 1.0)
    (bind _result (Math|Integer|IncrementInt _playerlevel_3)
      (:%20%20
        (Utilities|Array|SetArrayElem (Variables|Default|GetS_Attributos) 4 (Utilities|Struct|MakeS_Attributos "" 1 0.0 "" 0 _playername_3 _result))))
    (else
      (Utilities|Array|SetArrayElem (Variables|Default|GetS_Attributos) 4 (Utilities|Struct|MakeS_Attributos "" 1 0.0 "" 0 _playername_2 _playerlevel_2 _returnvalue_3))))
  (if (>= _returnvalue_4 1.0)
    (bind _result_2 (Math|Integer|IncrementInt _level)
      (:%20%20
        (Utilities|Array|SetArrayElem (Variables|Default|GetS_Attributos) (Variables|Default|GetIndex) (Utilities|Struct|MakeS_Attributos _name _result_2 0.0 _upgrade _expupgrade "None"))))
    (else
      (Utilities|Array|SetArrayElem (Variables|Default|GetS_Attributos) (Variables|Default|GetIndex) (Utilities|Struct|MakeS_Attributos _name _level _returnvalue_4 _upgrade _expupgrade _playername _playerlevel _playerexp)))))