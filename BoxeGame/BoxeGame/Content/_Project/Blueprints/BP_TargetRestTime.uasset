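; Timed target actor that scales its skeletal mesh in through a timeline and removes itself after a short lifetime or when its sphere is overlapped.
; BeginPlay caches the WB_Target widget, starts its animation and the timeline, then unhides the widget component when scaling finishes and waits briefly before destruction.
; A DestroyActor function destroys the actor and spawns a small lightning particle burst at its location.
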(event OnComponentBeginOverlap(Sphere)
  (params (OverlappedComponent :type Primitive%20Component%20Object%20Reference) (OtherActor :type Actor%20Object%20Reference) (OtherComp :type Primitive%20Component%20Object%20Reference) (OtherBodyIndex :type Integer) (bFromSweep :type Boolean) (SweepResult :type Hit%20Result%20Structure%20%28by%20ref%29))
  (CallFunction|DestroyActor))

(event EventBeginPlay
  (bind _aswb_target (Utilities|Casting|CastToWB_Target (UserInterface|GetWidget (Variables|Default|GetWidget))))
  (bind _output_get (Variables|Default|SetWB%20TargetRef _aswb_target))
  (UserInterface|Animation|PlayAnimation _output_get (Variables|/Game/_Project/UI/WB_Target.WB_Target_C|GetNewAnimation _output_get) 0.0 1 "Forward" 1.0 false)
  (bind _alpha (Timeline|Timeline_0 PlayFromStart)
    (:Update
      (Transformation|SetWorldScale3D (Variables|SkeletalMeshActor|GetSkeletalMeshComponent) (Math|Vector|MakeVector _alpha _alpha _alpha)))
    (:Finished
      (Development|SetHiddeninGame (Variables|Default|GetWidget) false false)
      (Utilities|FlowControl|Delay 2.0)
      (CallFunction|DestroyActor))))

(fn ConstructionScript)

(fn DestroyActor
  (Actor|DestroyActor)
  (Effects|SpawnEmitteratLocation "/Game/FXVarietyPack/Particles/P_ky_lightning1.P_ky_lightning1" (Transformation|GetActorLocation) "0, 0, 0" "0.200000,0.200000,0.200000"))