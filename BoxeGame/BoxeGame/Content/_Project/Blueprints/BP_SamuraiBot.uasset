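; Samurai enemy bot for a VR game, a child Blueprint that drives its animation state through AnimBP_Samurai.
; BeginPlay retries the anim-instance cast until it succeeds, and round start runs a timeline height adjustment on the mesh and enables target summoning.
; A melee hit switches animation and, outside placebo mode, stops movement.
; Punch-count reset, sword-slash montage and randomized AI movement timers are disconnected and never run.
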(event Custom|ChangeSamuraiCondition
  (params (Condition :type EN_Direction%20Enum :default "NewEnumerator0"))
  (Variables|/Game/SAM/DEMO/Mannequin/Animations/AnimBP_Samurai.AnimBP_Samurai_C|SetCurrentAnim (Variables|Default|GetAnim%20BP%20Samurai) Condition))

(event Custom|SamuraiHeightAdjustments
  (bind _mesh (Variables|Character|GetMesh))
  (bind _returnvalue (Transformation|GetWorldLocation _mesh))
  (bind _alpha (Timeline|Timeline_0 PlayFromStart)
    (:Update
      (Transformation|SetWorldLocation (Variables|Character|GetMesh) (Math|Vector|Lerp(Vector) (Transformation|GetWorldLocation _mesh) (Math|Vector|MakeVector (.x _returnvalue) (.y _returnvalue) 0.0) _alpha) false false))))

(event Custom|MeeleHit
  ;[1 1 1] MeeleAtack
  (Variables|/Game/SAM/DEMO/Mannequin/Animations/AnimBP_Samurai.AnimBP_Samurai_C|SetCurrentAnim (Variables|Default|GetAnim%20BP%20Samurai) "NewEnumerator3")
  (if (not (Variables|/Game/_Project/Framework/BP_GameInstance.BP_GameInstance_C|GetIsPlacebo (CallFunction|GetBoxegameInstance)))
    (Components|Movement|StopMovementImmediately (Variables|Character|GetCharacterMovement))
    (bind _asvrpawn (Utilities|Casting|CastToVRPawn (Game|Player|GetPlayerPawn 0)))))

(event EventBeginPlay
  (|CallParentFunction)
  (bind _asanim_bp_samurai (Utilities|Casting|CastToAnimBP_Samurai (Components|SkeletalMesh|GetAnimInstance (Variables|Default|GetSkeletalMesh)) :!label _label)
    (:then
      (bind _output_get (Variables|Default|SetAnim%20BP%20Samurai _asanim_bp_samurai))
      (Variables|/Game/SAM/DEMO/Mannequin/Animations/AnimBP_Samurai.AnimBP_Samurai_C|SetCurrentAnim _output_get "NewEnumerator1"))
    (:CastFailed
      (Utilities|FlowControl|Delay 0.2)
      (goto _label))))

(event EventOnStartSession
  (|CallParentFunction)
  (Development|PrintString "AI MOVE RECEIVING DISPATACHER" true true "(R=0.000000,G=0.660000,B=1.000000,A=1.000000)" 1e+03))

(fn ConstructionScript
  (Class|SkeletalMeshComponent|SetAnimClass (Variables|Default|GetSkeletalMesh) "/Game/SAM/DEMO/Mannequin/Animations/AnimBP_Samurai.AnimBP_Samurai_C"))

(fn SetuponStartRound
  (CallFunction|SamuraiHeightAdjustments)
  (Variables|Default|SetCanSummonTargets? true))