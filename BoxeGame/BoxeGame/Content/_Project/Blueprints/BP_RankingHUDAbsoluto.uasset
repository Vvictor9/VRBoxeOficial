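; BP_RankingHUDAbsoluto hosts a WBP_RankingAbsoluto widget through a Widget component to display the absolute ranking.
; On BeginPlay it polls every second until the Boxegame instance is valid, then binds to its OnUpdateRank event, caches the widget and refreshes it.
; AtualizarValores refreshes the cached widget's rank values, passing the IsLast20 flag instead of the false used on startup.
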(event EventBeginPlay
  (bind _boxegameinstance (CallFunction|GetBoxegameInstance))
  (Utilities|IsValid _boxegameinstance :!label _label
    (:Is%20Valid
      (EventDispatchers|BindEventtoOnUpdateRank _boxegameinstance (EventDispatchers|CreateEvent :!event AtualizarValores))
      (bind _aswbp_ranking_absoluto (Utilities|Casting|CastToWBP_RankingAbsoluto (UserInterface|GetWidget (Variables|Default|GetWidget))))
      (bind _output_get (Variables|Default|SetHUD%20RankingInstance _aswbp_ranking_absoluto))
      (Default|AtualizarValorRank _output_get false))
    (:Is%20Not%20Valid
      (Utilities|FlowControl|Delay 1.0)
      (goto _label))))

(fn ConstructionScript)

(fn AtualizarValores
  (bind _hud_rankinginstance (Variables|Default|GetHUD%20RankingInstance)
    (:then
      (Default|AtualizarValorRank _hud_rankinginstance (Variables|Config|GetIsLast20)))
    (:else)))