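; BP_Shuriken is a thrown shuriken projectile for the VR player that damage-free registers hits on BP_PhysicalAnimTest actors.
; The OnShotShuriken event starts a timeline that moves it along its spline, then destroys it after a short delay.
; Tick continuously spins the mesh in yaw with interpolated rotation.
; A box overlap plays a hit sound, destroys the shuriken, increments VRPawn's hit count and charges mana.
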(event OnComponentBeginOverlap(Box)
  (params (OverlappedComponent :type Primitive%20Component%20Object%20Reference) (OtherActor :type Actor%20Object%20Reference) (OtherComp :type Primitive%20Component%20Object%20Reference) (OtherBodyIndex :type Integer) (bFromSweep :type Boolean) (SweepResult :type Hit%20Result%20Structure%20%28by%20ref%29))
  (bind _vrpawnref (Variables|Default|GetVRPawnRef))
  (bind _bpc_timer (Variables|/Game/_Project/Blueprints/VRPawn.VRPawn_C|GetBPC_Timer _vrpawnref))
  (bind _asbp_physical_anim_test (Utilities|Casting|CastToBP_PhysicalAnimTest OtherActor))
  (Audio|SpawnSoundatLocation "/Game/_Project/Blueprints/Shuriken/Sound/ShurikenHit.ShurikenHit" (Transformation|GetActorLocation _asbp_physical_anim_test) "0, 0, 0" 1.0 1.0 0.0 0 0)
  (Actor|DestroyActor)
  (Default|IncreaseNumHitsonRestTime (Variables|Default|GetVRPawnRef))
  (Default|ChargeMana _bpc_timer (Default|ReturnManatoCharge _bpc_timer)))

(event Custom|ShotShuriken
  (bind _alpha (Timeline|TL_ShotShuriken PlayFromStart)
    (:Update
      (Transformation|SetActorLocation (Spline|GetLocationatDistanceAlongSpline (Variables|Default|GetSpline) (Math|Float|Lerp 0.0 (Spline|GetSplineLength (Variables|Default|GetSpline)) _alpha) "World") false false))
    (:Finished
      (Utilities|FlowControl|Delay 3.0)
      (Actor|DestroyActor))))

(event EventBeginPlay
  (bind _asvrpawn (Utilities|Casting|CastToVRPawn (Game|Player|GetPlayerPawn 0)))
  (Variables|Default|SetVRPawnRef _asvrpawn)
  (EventDispatchers|BindEventtoOnShotShuriken (delegate Custom|ShotShuriken)))

(event EventTick
  (params (DeltaSeconds :type Float%20%28single-precision%29))
  (Transformation|SetWorldRotation (Variables|Default|GetSM_Shuriken) (Math|Interpolation|RInterpTo (Transformation|GetWorldRotation (Variables|Default|GetSM_Shuriken)) (Math|Rotator|MakeRotator (Variables|Default|GetX%20%28Roll%29) 0.0 (+ (.yaw (Transformation|GetWorldRotation (Variables|Default|GetSM_Shuriken))) 8.0)) DeltaSeconds (Variables|Default|GetInterp%20Speed)) false false))

(fn ConstructionScript)