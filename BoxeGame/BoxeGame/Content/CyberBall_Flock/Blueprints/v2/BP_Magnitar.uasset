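; BP_Magnitar is a magnet-like field actor that pushes or pulls nearby objects by firing a RadialForce impulse every tick.
; The construction script copies the Radius and ImpulseStrength variables onto the RadialForce component and gives the Sphere a dynamic material.
; That material's speed follows the signed strength, and its two colors turn orange for positive values, blue otherwise.
; An older material setup in the event graph is left unconnected.
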(event EventBeginPlay)

(event Collision|EventActorBeginOverlap
  (params (OtherActor :type Actor%20Object%20Reference)))

(event EventTick
  (params (DeltaSeconds :type Float%20%28single-precision%29))
  (Class|RadialForceComponent|FireImpulse (Variables|Default|GetRadialForce)))

(fn ConstructionScript
  (bind _radialforce (Variables|Default|GetRadialForce))
  (Variables|/Script/Engine.RadialForceComponent|SetRadius _radialforce (Variables|Default|GetRadius))
  (Variables|/Script/Engine.RadialForceComponent|SetImpulseStrength _radialforce (Variables|Default|GetImpulse%20Strength))
  (bind _returnvalue (Rendering|Material|CreateDynamicMaterialInstance (Rendering|Material|GetMaterial (Variables|Default|GetSphere) 0) "Mat_dyn_instance" "None" :!class /Script/Engine.KismetMaterialLibrary))
  (Rendering|Material|SetMaterial (Variables|Default|GetSphere) 0 _returnvalue)
  (Rendering|Material|SetScalarParameterValue _returnvalue "speed" (Math|Float|MapRangeClamped (Variables|/Script/Engine.RadialForceComponent|GetImpulseStrength (Variables|Default|GetRadialForce)) -3e+04 3e+04 -1e+01 1e+01) :!class /Script/Engine.MaterialInstanceDynamic)
  (if (> (Variables|/Script/Engine.RadialForceComponent|GetImpulseStrength (Variables|Default|GetRadialForce)) 0.0)
    (Rendering|Material|SetVectorParameterValue _returnvalue "Color1" "(R=1.000000,G=0.644330,B=0.000000,A=1.000000)" :!class /Script/Engine.MaterialInstanceDynamic)
    (Rendering|Material|SetVectorParameterValue _returnvalue "Color2" "(R=0.703125,G=0.074849,B=0.000000,A=1.000000)" :!class /Script/Engine.MaterialInstanceDynamic)
    (else
      (Rendering|Material|SetVectorParameterValue _returnvalue "Color1" "(R=0.000000,G=0.728769,B=1.000000,A=1.000000)" :!class /Script/Engine.MaterialInstanceDynamic)
      (Rendering|Material|SetVectorParameterValue _returnvalue "Color2" "(R=0.034151,G=0.000000,B=1.000000,A=1.000000)" :!class /Script/Engine.MaterialInstanceDynamic))))