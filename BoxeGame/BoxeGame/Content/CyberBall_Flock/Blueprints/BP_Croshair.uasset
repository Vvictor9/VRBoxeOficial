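; BP_Croshair is a HUD Blueprint that draws a small dot crosshair at the center of the screen.
; Each DrawHUD call casts player character 0 to TPS_CyberBalls_Flock_V2 and draws only while that character's Croshair flag is set.
; The dot is green while the character's AltIsPressed flag is true and red otherwise.
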(event EventDrawHUD
  (params (SizeX :type Integer) (SizeY :type Integer))
  (bind _returnvalue (/ SizeX 2))
  (bind _returnvalue_2 (/ SizeY 2))
  (bind _self self)
  (bind _returnvalue_3 (Math|Conversions|ToFloat(Integer) _returnvalue_2))
  (bind _returnvalue_4 (Math|Conversions|ToFloat(Integer) _returnvalue))
  (bind _astps_cyber_balls_flock_v2 (Utilities|Casting|CastToTPS_CyberBalls_Flock_V2 (Game|GetPlayerCharacter 0)))
  (if (Variables|/Game/CyberBall_Flock/Blueprints/v2/TPS_CyberBalls_Flock_V2.TPS_CyberBalls_Flock_V2_C|GetCroshair _astps_cyber_balls_flock_v2)
    (if (Variables|/Game/CyberBall_Flock/Blueprints/v2/TPS_CyberBalls_Flock_V2.TPS_CyberBalls_Flock_V2_C|Getalt%20is%20pressed _astps_cyber_balls_flock_v2)
      (HUD|DrawRect _self "(R=0.000000,G=1.000000,B=0.041187,A=1.000000)" _returnvalue_4 _returnvalue_3 3.0 3.0)
      (else
        (HUD|DrawRect _self "(R=1.000000,G=0.000000,B=0.102203,A=1.000000)" _returnvalue_4 _returnvalue_3 3.0 3.0)))))

(fn ConstructionScript)