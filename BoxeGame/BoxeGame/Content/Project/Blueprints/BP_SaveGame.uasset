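; BP_SaveGame holds a top-ten ranking of values and provides functions to update and reset it.
; AddNewValue sorts the list descending through OrganizeArray's selection sort, then appends a qualifying value and removes index 9, the previous lowest.
; The list is not re-sorted after insertion, so the new entry stays last until the next sort.
; ResetSaveValues refills the ranking with ten zeros.
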(fn AddNewValue
  (params (NewValue :type Integer))
  (bind _rankingvalues (Variables|Default|GetRankingValues))
  (CallFunction|OrganizeArray)
  (bind _array_element (Utilities|Array|ForEachLoopwithBreak (Variables|Default|GetRankingValues) :!label _label)
    (:LoopBody
      (if (<= _array_element NewValue)
        (Utilities|Array|Add _rankingvalues NewValue)
        (Utilities|Array|RemoveIndex _rankingvalues 9)
        (goto _label Break)))))

(fn ResetSaveValues
  (Variables|Default|SetRankingValues (Utilities|Array|MakeArray 0 0 0 0 0 0 0 0 0 0)))

(fn OrganizeArray
  (bind _rankingvalues (Variables|Default|GetRankingValues))
  (bind _returnvalue (Utilities|Array|Length _rankingvalues))
  (bind _returnvalue_2 (- _returnvalue 1))
  (for _index (range 0 _returnvalue_2)
    (LocalVariables|SetCurrentBiggerValue (Utilities|Array|Get(acopy) (Variables|Default|GetRankingValues) _index))
    (LocalVariables|SetCurrentBiggerIndex _index)
    (for _index_2 (range (+ _index 1) _returnvalue_2)
      (if (>= (Utilities|Array|Get(acopy) (Variables|Default|GetRankingValues) _index_2) (LocalVariables|GetCurrentBiggerValue))
        (LocalVariables|SetCurrentBiggerValue (Utilities|Array|Get(acopy) (Variables|Default|GetRankingValues) _index_2))
        (LocalVariables|SetCurrentBiggerIndex _index_2)))
    (LocalVariables|SetAuxValor (Utilities|Array|Get(acopy) (Variables|Default|GetRankingValues) _index))
    (Utilities|Array|SetArrayElem (Variables|Default|GetRankingValues) _index (LocalVariables|GetCurrentBiggerValue))
    (Utilities|Array|SetArrayElem (Variables|Default|GetRankingValues) (LocalVariables|GetCurrentBiggerIndex) (LocalVariables|GetAuxValor))))