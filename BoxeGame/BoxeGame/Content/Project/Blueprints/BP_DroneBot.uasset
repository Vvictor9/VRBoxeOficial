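; Flying drone punching target that circles the player while always facing them.
; Glove overlaps fire OnPunchBag with the hand side, plus a backward bone impulse, metal sound and firework Niagara burst; per-glove flags block repeat hits until overlap ends.
; After a startup delay, recursive AIMoveTo side steps along the right vector create the orbit while CanMove holds, with random pauses and reversals, feeding direction to the AnimBP.
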(event OnComponentEndOverlap(DroneOverlap)
  (params (OverlappedComponent :type Primitive%20Component%20Object%20Reference) (OtherActor :type Actor%20Object%20Reference) (OtherComp :type Primitive%20Component%20Object%20Reference) (OtherBodyIndex :type Integer))
  (bind _returnvalue (Utilities|GetObjectName OtherComp))
  (if (Utilities|Enum|Equal(Enum) _returnvalue "SC_GloveR")
    (Variables|Default|SetFlagRDontEndOverlapYet false)
    (elif (Utilities|Enum|Equal(Enum) _returnvalue "SC_GloveL")
      (Variables|Default|SetFlagLDontEndOverlapYet false))))

(event OnComponentBeginOverlap(Overlap)
  (params (OverlappedComponent :type Primitive%20Component%20Object%20Reference) (OtherActor :type Actor%20Object%20Reference) (OtherComp :type Primitive%20Component%20Object%20Reference) (OtherBodyIndex :type Integer) (bFromSweep :type Boolean) (SweepResult :type Hit%20Result%20Structure%20%28by%20ref%29))
  (bind _returnvalue (Utilities|GetObjectName OtherComp))
  (bind _returnvalue_2 (Transformation|GetWorldLocation OtherComp))
  (bind _droneoverlap (Variables|Default|GetDroneOverlap))
  (bind _returnvalue_3 (Transformation|GetWorldLocation _droneoverlap))
  (bind _returnvalue_4 (- _returnvalue_3 _returnvalue_2))
  (bind _returnvalue_5 (Math|Vector|Normalize _returnvalue_4))
  (bind _returnvalue_6 (* _returnvalue_5 15.0))
  (bind _returnvalue_7 (+ _returnvalue_2 _returnvalue_6))
  (if (Utilities|Enum|Equal(Enum) _returnvalue "SC_GloveR")
    (if (not (Variables|Default|GetFlagRDontEndOverlapYet))
      (Variables|Default|SetFlagRDontEndOverlapYet true)
      (Default|CallOnPunchBag true)
      (Physics|AddImpulseatLocation (Variables|Default|GetSkeletalMesh) (* (* (Math|Vector|GetForwardVector (Variables|Default|GetSkeletalMesh)) -1.0) 1e+03) (.Location (Collision|BreakHitResult SweepResult)) "DronBot" :!label _label)
      (Audio|PlaySoundatLocation "/Game/Project/Sounds/GameplaySounds/MetalSound.MetalSound" (Transformation|GetWorldLocation OtherComp) "0, 0, 0" 0.7 1.0 0.0 0 0 0)
      (Niagara|SpawnSystematLocation "/Game/Project/NiagaraAbstractSpace3/Effects/NS_Sphere_of_Fireworks.NS_Sphere_of_Fireworks" (Math|Vector|MakeVector (.x _returnvalue_7) (.y _returnvalue_7) (.z (Transformation|GetWorldLocation OtherComp)))))
    (elif (Utilities|Enum|Equal(Enum) _returnvalue "SC_GloveL")
      (if (not (Variables|Default|GetFlagLDontEndOverlapYet))
        (Variables|Default|SetFlagLDontEndOverlapYet true)
        (Default|CallOnPunchBag false)
        (goto _label)))))

(event Custom|AiMovement
  (params (HorarioCycle :type Boolean))
  ;[1 1 1] Movement
  (Variables|/Game/Project/Meshs/AnimBP_Drone.AnimBP_Drone_C|SetCurrentDirection (Variables|Default|GetAnim%20BP%20Drone) (select HorarioCycle "NewEnumerator2" "NewEnumerator1"))
  (if (Variables|Config|GetCanMove)
    (AI|AIMoveTo self (+ (Transformation|GetActorLocation) (* (Transformation|GetActorRightVector) (select HorarioCycle 5e+01 -5e+01))) 0 1.0 false
      (:OnSuccess
        _)
      (:OnFail
        _))
    (if (>= (Math|Random|RandomFloat) 0.9)
      (Variables|/Game/Project/Meshs/AnimBP_Drone.AnimBP_Drone_C|SetCurrentDirection (Variables|Default|GetAnim%20BP%20Drone) "NewEnumerator0")
      (Utilities|FlowControl|Delay (Math|Random|RandomFloatinRange 2.0 5.0)))
    (CallFunction|AiMovement (select (>= (Math|Random|RandomFloat) 0.05) HorarioCycle (not HorarioCycle)))))

(event EventBeginPlay
  (Utilities|FlowControl|Delay 3.0)
  (bind _asanim_bp_drone (Utilities|Casting|CastToAnimBP_Drone (Components|SkeletalMesh|GetAnimInstance (Variables|Default|GetSkeletalMesh))))
  (Variables|Default|SetAnim%20BP%20Drone _asanim_bp_drone)
  (Pawn|Components|CharacterMovement|SetMovementMode (Variables|Character|GetCharacterMovement) "MOVE_Flying" 0)
  (CallFunction|AiMovement (Math|Random|RandomBool)))

(event EventTick
  (params (DeltaSeconds :type Float%20%28single-precision%29))
  (Transformation|SetActorRotation (Math|Rotator|MakeRotator 0.0 0.0 (.yaw (Math|Rotator|FindLookatRotation (Transformation|GetActorLocation) (Transformation|GetActorLocation (Pawn|GetControlledPawn (Game|GetPlayerController 0))))))))

(fn ConstructionScript)