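; HUD controller component on the VR pawn that runs a boxing round of alternating punch and rest intervals.
; StartRound resets the WI_BattleTime widget, then looping timers drive the interval counters and loading bars, with alert sounds at transitions.
; Punches and glove-boosted speed reach the widget only while counting is unblocked during punch intervals.
; After twelve punch sessions it records the total in the game instance and finishes the round.
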(event EventBeginPlay
  (bind _asvrpawn (Utilities|Casting|CastToVRPawn (Components|GetOwner)))
  (Variables|Default|SetOwnerRef _asvrpawn)
  (bind _aswi_battle_time (Utilities|Casting|CastToWI_BattleTime (UserInterface|GetWidget (Variables|/Game/Project/Blueprints/VRPawn.VRPawn_C|GetHUD _asvrpawn))))
  (Variables|Default|SetWidgetRef _aswi_battle_time)
  (Default|SetPunchValue _aswi_battle_time))

(fn StartRound
  (Variables|Default|SetQuantPunchSessions 1)
  (Variables|Default|SetTimerCurrentValue 0)
  (Variables|Default|SetPunchValue 0)
  (Variables|/Game/Project/UI/WI_BattleTime.WI_BattleTime_C|SetCountRing (Variables|Default|GetWidgetRef) 0)
  (Variables|/Game/Project/UI/WI_BattleTime.WI_BattleTime_C|SetCountReload (Variables|Default|GetWidgetRef) 0)
  (Variables|/Game/Project/UI/WI_BattleTime.WI_BattleTime_C|SetCountReady (Variables|Default|GetWidgetRef) 0)
  (Variables|/Game/Project/UI/WI_BattleTime.WI_BattleTime_C|SetCountUnLoadingBar (Variables|Default|GetWidgetRef) 40)
  (Variables|/Game/Project/UI/WI_BattleTime.WI_BattleTime_C|SetCountLoadingBar (Variables|Default|GetWidgetRef) 0)
  (Default|SetPunchValue (Variables|Default|GetWidgetRef))
  (Variables|Default|SetIsSecondTimerPunch false)
  (Default|InitStartTimer (Variables|Default|GetWidgetRef))
  (Utilities|Time|SetTimerbyEvent (EventDispatchers|CreateEvent :!event StartPunchTimer) 5.0))

(fn StartRestTimer
  (Variables|Default|SetTimerCurrentValue 0)
  (CallFunction|BlockPunchCount)
  (Default|StartRestTime (Variables|Default|GetWidgetRef) (Variables|Default|GetQuantPunchSessions))
  (bind _returnvalue (Utilities|Time|SetTimerbyEvent (EventDispatchers|CreateEvent :!event UpdateTimerRest) 1.0 true))
  (Variables|Default|SetTimer_Timer _returnvalue)
  (Utilities|Time|SetTimerbyFunctionName (Variables|Default|GetWidgetRef) "InitLoadingBarTimer" 0.4 true 2.0)
  (Audio|PlaySound2D "/Game/Project/Sounds/Alert_Cue.Alert_Cue" 1.0 1.0 0.0 0 0))

(fn StartPunchTimer
  (Audio|PlaySound2D "/Game/Project/Sounds/Alert_Cue.Alert_Cue" 1.0 1.0 0.0 0 0)
  (Variables|Default|SetTimerCurrentValue 0)
  (Utilities|FlowControl|Sequence
    (:then_0
      (CallFunction|UnlockPunchCount false)
      (bind _returnvalue (Utilities|Time|SetTimerbyEvent (EventDispatchers|CreateEvent :!event UpdateTimerPunch) 1.0 true))
      (Variables|Default|SetTimer_Timer _returnvalue)
      (Utilities|Time|SetTimerbyFunctionName (Variables|Default|GetWidgetRef) "InitUnloadingBarTimer" 0.32 true 2.0))
    (:then_1
      (if (Variables|Default|GetIsSecondTimerPunch)
        (Default|StartPunchTime (Variables|Default|GetWidgetRef))))))

(fn UpdateTimerPunch
  (bind _output_get (Variables|Default|SetTimerCurrentValue (+ (Variables|Default|GetTimerCurrentValue) 1)))
  (if (>= _output_get (Variables|Default|GetMaxTimerPunch))
    (CallFunction|StopTimerPunch)))

(fn UpdateTimerRest
  (bind _output_get (Variables|Default|SetTimerCurrentValue (+ (Variables|Default|GetTimerCurrentValue) 1)))
  (if (>= _output_get (Variables|Default|GetMaxTimerRest))
    (CallFunction|StopTimerRest)))

(fn StopTimerRest
  (Utilities|Time|ClearandInvalidateTimerbyHandle (Variables|Default|GetTimer_Timer))
  (CallFunction|BlockPunchCount)
  (Variables|Default|SetIsSecondTimerPunch true)
  (CallFunction|StartPunchTimer))

(fn StopTimerPunch
  (Utilities|Time|ClearandInvalidateTimerbyHandle (Variables|Default|GetTimer_Timer))
  (CallFunction|BlockPunchCount)
  (bind _output_get (Variables|Default|SetQuantPunchSessions (+ (Variables|Default|GetQuantPunchSessions) 1)))
  (if (>= _output_get 13)
    ;[1 1 1] Finish round save punch numbers in save
    (Default|AddNewValue (CallFunction|GetBoxegameInstance) (Variables|Default|GetPunchValue))
    (Default|FinishRound (Variables|Default|GetWidgetRef))
    (Audio|PlaySound2D "/Game/Project/Sounds/Alert_Cue.Alert_Cue" 1.0 1.0 0.0 0 0)
    (else
      (CallFunction|StartRestTimer))))

(fn AddPunchValue
  (if (not (Variables|Default|GetIsBlockingPunch))
    (bind _widgetref (Variables|Default|GetWidgetRef)
      (:then
        (bind _result (Math|Integer|IncrementInt (Variables|Default|GetPunchValue))
          (:%20%20
            (Default|SetPunchValue _widgetref _result)
            (if (> (Variables|/Game/Project/Blueprints/VRPawn.VRPawn_C|GetPunchSpeedValue (Variables|Default|GetOwnerRef)) 0.0)
              (Default|SetPunchSpeed (Variables|Default|GetWidgetRef) (* (Variables|/Game/Project/Blueprints/VRPawn.VRPawn_C|GetPunchSpeedValue (Variables|Default|GetOwnerRef)) (Variables|Default|GetGloveBooster)))))))
      (:else))))

(fn BlockPunchCount
  (Variables|Default|SetIsBlockingPunch true))

(fn UnlockPunchCount
  (params (ResetValue :type Boolean))
  (Variables|Default|SetIsBlockingPunch false)
  (if ResetValue
    (Default|SetPunchValue (Variables|Default|GetWidgetRef) (Variables|Default|GetPunchValue))))