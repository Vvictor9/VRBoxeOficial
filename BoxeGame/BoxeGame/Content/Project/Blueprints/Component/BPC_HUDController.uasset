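; HUD controller component for a VR boxing round, running alternating punch and rest intervals and tracking the punch score.
; On BeginPlay it retries until it finds the VR pawn's WI_BattleTime widget, which it drives with countdowns, loading bars and score.
; Looping timers switch phases with alert sounds, and points count only during punch phases.
; After twelve punch sessions it saves the score to the game instance and re-enables pawn input.
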(event EventBeginPlay
  (bind _asvrpawn (Utilities|Casting|CastToVRPawn (Pawn|GetControlledPawn (Game|GetPlayerController 0))))
  (Variables|Default|SetOwnerRef _asvrpawn)
  (bind _aswi_battle_time (Utilities|Casting|CastToWI_BattleTime (UserInterface|GetWidget (Variables|/Game/Project/Blueprints/VRPawn.VRPawn_C|GetHUD _asvrpawn)) :!label _label)
    (:then
      (bind _output_get (Variables|Default|SetWidgetRef _aswi_battle_time))
      (Default|SetPunchValue _output_get))
    (:CastFailed
      (Utilities|FlowControl|Delay 0.5)
      (goto _label))))

(fn StartRound
  (Variables|Timer|SetQuantPunchSessions 1)
  (Variables|Default|SetTimerCurrentValue 0)
  (Variables|Default|SetPunchValue 0)
  (Variables|/Game/Project/UI/WI_BattleTime.WI_BattleTime_C|SetCountRing (Variables|Default|GetWidgetRef) 0)
  (Variables|/Game/Project/UI/WI_BattleTime.WI_BattleTime_C|SetCountReload (Variables|Default|GetWidgetRef) 0)
  (Variables|/Game/Project/UI/WI_BattleTime.WI_BattleTime_C|SetCountReady (Variables|Default|GetWidgetRef) 0)
  (Variables|/Game/Project/UI/WI_BattleTime.WI_BattleTime_C|SetCountUnLoadingBar (Variables|Default|GetWidgetRef) 40)
  (Variables|/Game/Project/UI/WI_BattleTime.WI_BattleTime_C|SetCountLoadingBar (Variables|Default|GetWidgetRef) 0)
  (Default|SetPunchValue (Variables|Default|GetWidgetRef))
  (Variables|Default|SetIsSecondTimerPunch false)
  (Default|InitStartTimer (Variables|Default|GetWidgetRef))
  (Utilities|Time|SetTimerbyEvent (EventDispatchers|CreateEvent :!event StartPunchTimer) 3.0))

(fn StartRestTimer
  (Variables|Default|SetTimerCurrentValue 0)
  (CallFunction|BlockPunchCount)
  (Default|StartRestTime (Variables|Default|GetWidgetRef) (Variables|Timer|GetQuantPunchSessions))
  (bind _returnvalue (Utilities|Time|SetTimerbyEvent (EventDispatchers|CreateEvent :!event UpdateTimerRest) 1.0 true))
  (Variables|Default|SetTimer_Timer _returnvalue)
  (Default|InitLoadingBarTimer (Variables|Default|GetWidgetRef) 0.5)
  (Audio|PlaySound2D "/Game/Project/Sounds/Alert_Cue.Alert_Cue" 1.0 1.0 0.0 0 0)
  (Default|CallStartRestTime))

(fn StartPunchTimer
  (Audio|PlaySound2D "/Game/Project/Sounds/Alert_Cue.Alert_Cue" 1.0 1.0 0.0 0 0)
  (Variables|Default|SetTimerCurrentValue 0)
  (Utilities|FlowControl|Sequence
    (:then_0
      (if (Variables|Default|GetIsSecondTimerPunch)
        (Variables|Default|SetTimeToUnloading 3.0)
        (Default|StartPunchTime (Variables|Default|GetWidgetRef))))
    (:then_1
      (CallFunction|UnlockPunchCount false)
      (bind _returnvalue (Utilities|Time|SetTimerbyEvent (EventDispatchers|CreateEvent :!event UpdateTimerPunch) 1.0 true))
      (Variables|Default|SetTimer_Timer _returnvalue)
      (if (Variables|Default|GetIsSecondTimerPunch)
        (bind _returnvalue_2 (Utilities|Time|SetTimerbyFunctionName (Variables|Default|GetWidgetRef) "InitUnloadingBarTimer" (Variables|Default|GetTimeToUnloading)))
        (Variables|Default|SetTHUnLoadingBarAnimation _returnvalue_2)
        (else
          (Default|InitUnLoadingBarTimer (Variables|Default|GetWidgetRef)))))
    (:then_2
      (Default|CallStartPunchTime))))

(fn UpdateTimerPunch
  (bind _output_get (Variables|Default|SetTimerCurrentValue (+ (Variables|Default|GetTimerCurrentValue) 1)))
  (if (>= _output_get (Variables|Timer|GetMaxTimerPunch))
    (CallFunction|StopTimerPunch)))

(fn UpdateTimerRest
  (bind _output_get (Variables|Default|SetTimerCurrentValue (+ (Variables|Default|GetTimerCurrentValue) 1)))
  (if (>= _output_get (Variables|Timer|GetMaxTimerRest))
    (CallFunction|StopTimerRest)))

(fn StopTimerRest
  (Utilities|Time|ClearandInvalidateTimerbyHandle (Variables|Default|GetTimer_Timer))
  (Utilities|Time|ClearandInvalidateTimerbyHandle (Variables|Default|GetTHloadingBarAnimation))
  (CallFunction|BlockPunchCount)
  (Variables|Default|SetIsSecondTimerPunch true)
  (CallFunction|StartPunchTimer))

(fn StopTimerPunch
  (Utilities|Time|ClearandInvalidateTimerbyHandle (Variables|Default|GetTimer_Timer))
  (Utilities|Time|ClearandInvalidateTimerbyHandle (Variables|Default|GetTHUnLoadingBarAnimation))
  (CallFunction|BlockPunchCount)
  (bind _output_get (Variables|Timer|SetQuantPunchSessions (+ (Variables|Timer|GetQuantPunchSessions) 1)))
  (if (>= _output_get 13)
    ;[1 1 1] Finish round save punch numbers in save
    (Default|AddNewValue (CallFunction|GetBoxegameInstance) (Variables|Default|GetPunchValue))
    (Default|FinishRound (Variables|Default|GetWidgetRef))
    (Audio|PlaySound2D "/Game/Project/Sounds/Alert_Cue.Alert_Cue" 1.0 1.0 0.0 0 0)
    (Input|EnableInput (Pawn|GetControlledPawn (Game|GetPlayerController 0)) (Game|GetPlayerController 0))
    (else
      (CallFunction|StartRestTimer))))

(fn AddPunchValue
  (params (Points :type Float%20%28single-precision%29))
  (if (not (Variables|Default|GetIsBlockingPunch))
    (bind _widgetref (Variables|Default|GetWidgetRef)
      (:then
        (bind _output_get (Variables|Default|SetPunchValue (+ (Variables|Default|GetPunchValue) (Math|Float|Truncate Points))))
        (Default|SetPunchValue _widgetref _output_get))
      (:else))))

(fn BlockPunchCount
  (Variables|Default|SetIsBlockingPunch true))

(fn UnlockPunchCount
  (params (ResetValue :type Boolean))
  (Variables|Default|SetIsBlockingPunch false)
  (if ResetValue
    (Default|SetPunchValue (Variables|Default|GetWidgetRef) (Variables|Default|GetPunchValue))))