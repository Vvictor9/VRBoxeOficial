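; Punching bag actor that reacts to hits with physics, sound and effects.
; Overlap begin stops the Slerp timeline, resets the constraint's angular drive, plays a hit sound, spawns Niagara fireworks and fires the OnPunchBag dispatcher.
; The effect is offset horizontally from the hitting component toward the overlap volume, keeping the hit height.
; Overlap end plays the timeline, blending the drive to higher position strength and lower velocity strength.
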(event OnComponentBeginOverlap(Overlap)
  (params (OverlappedComponent :type Primitive%20Component%20Object%20Reference) (OtherActor :type Actor%20Object%20Reference) (OtherComp :type Primitive%20Component%20Object%20Reference) (OtherBodyIndex :type Integer) (bFromSweep :type Boolean) (SweepResult :type Hit%20Result%20Structure%20%28by%20ref%29))
  (bind _returnvalue (Transformation|GetWorldLocation OtherComp))
  (bind _overlap (Variables|Default|GetOverlap))
  (bind _returnvalue_2 (Transformation|GetWorldLocation _overlap))
  (bind _returnvalue_3 (- _returnvalue_2 _returnvalue))
  (bind _returnvalue_4 (Math|Vector|Normalize _returnvalue_3))
  (bind _returnvalue_5 (* _returnvalue_4 5e+01))
  (bind _returnvalue_6 (+ _returnvalue _returnvalue_5))
  ;[1 0 0.03471] Comportamento de reação das fisicas e effects do saco de pancada ao tomar golpes
  (Development|PrintString "SOCOU!" false false "(R=0.000000,G=0.660000,B=1.000000,A=1.000000)" 1.0)
  (Utilities|FlowControl|Sequence
    (:then_0
      (Audio|Components|Audio|Stop (Variables|Default|GetSlerp))
      (Class|PhysicsConstraintComponent|SetAngularDriveParams (Variables|Default|GetPhysicsConstraint) (Math|Float|MakeLiteralFloat 1e+02) (Math|Float|MakeLiteralFloat 3e+01) 0.0)
      (Audio|PlaySoundatLocation "/Game/Project/Sounds/hit_Cue.hit_Cue" (Transformation|GetWorldLocation OtherComp) "0, 0, 0" 1.0 1.0 0.0 0 0 0)
      (Niagara|SpawnSystematLocation "/Game/Project/NiagaraAbstractSpace3/Effects/NS_Sphere_of_Fireworks.NS_Sphere_of_Fireworks" (Math|Vector|MakeVector (.x _returnvalue_6) (.y _returnvalue_6) (.z (Transformation|GetWorldLocation OtherComp)))))
    (:then_1
      (Default|CallOnPunchBag))))

(event OnComponentEndOverlap(Overlap)
  (params (OverlappedComponent :type Primitive%20Component%20Object%20Reference) (OtherActor :type Actor%20Object%20Reference) (OtherComp :type Primitive%20Component%20Object%20Reference) (OtherBodyIndex :type Integer))
  ;[1 0 0.03471] Comportamento de reação das fisicas e effects do saco de pancada ao tomar golpes
  (Utilities|FlowControl|Sequence
    (:then_0
      (bind _alpha (Timeline|Slerp PlayFromStart)
        (:Update
          (Class|PhysicsConstraintComponent|SetAngularDriveParams (Variables|Default|GetPhysicsConstraint) (Math|Float|Lerp (Math|Float|MakeLiteralFloat 1e+02) 4e+02 _alpha) (Math|Float|Lerp (Math|Float|MakeLiteralFloat 3e+01) 1.0 _alpha) 0.0))))))

(fn ConstructionScript)