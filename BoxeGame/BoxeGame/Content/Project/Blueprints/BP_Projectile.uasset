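; Lightning-effect projectile that homes in on the player pawn, which can punch it for points or take a penalty when hit.
; Projectile movement targets the player's root on BeginPlay and is activated after a short delay.
; Capsule overlap plays the hit effect, disables collision, hides the shot effect and destroys the actor shortly after.
; For a VRPawn, the overlapped component's object channel selects left/right punch speed to add to BPCTimer, otherwise subtracting a fixed amount.
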(event OnComponentBeginOverlap(Capsule)
  (params (OverlappedComponent :type Primitive%20Component%20Object%20Reference) (OtherActor :type Actor%20Object%20Reference) (OtherComp :type Primitive%20Component%20Object%20Reference) (OtherBodyIndex :type Integer) (bFromSweep :type Boolean) (SweepResult :type Hit%20Result%20Structure%20%28by%20ref%29))
  (bind _returnvalue (Collision|GetCollisionObjectType OtherComp))
  (bind _returnvalue_2 (Utilities|Enum|Equal(Enum) _returnvalue "ECC_GameTraceChannel4"))
  (Utilities|FlowControl|Sequence
    (:then_0
      (Components|Activation|SetActive (Variables|Default|GetP_ky_hit_thunder) true true)
      (Collision|SetCollisionEnabled (Variables|Default|GetCapsule) "NoCollision")
      (Rendering|SetVisibility (Variables|Default|GetP_ky_shot_thunder) false false)
      (Utilities|FlowControl|Delay 1.0)
      (Actor|DestroyActor))
    (:then_1
      (bind _asvrpawn (Utilities|Casting|CastToVRPawn OtherActor))
      (if (or _returnvalue_2 (Utilities|Enum|Equal(Enum) _returnvalue "ECC_GameTraceChannel2"))
        (Default|AddPunchValue (Variables|/Game/Project/Blueprints/VRPawn.VRPawn_C|GetBPC_Timer _asvrpawn) (/ (Math|Float|SelectFloat (Variables|/Game/Project/Blueprints/VRPawn.VRPawn_C|GetPunchLSpeedValue _asvrpawn) (Variables|/Game/Project/Blueprints/VRPawn.VRPawn_C|GetPunchRSpeedValue _asvrpawn) _returnvalue_2) 3.0))
        (else
          (Default|AddPunchValue (Variables|/Game/Project/Blueprints/VRPawn.VRPawn_C|GetBPC_Timer _asvrpawn) -2e+02))))))

(event EventBeginPlay
  (Variables|/Script/Engine.ProjectileMovementComponent|SetHomingTargetComponent (Variables|Default|GetProjectileMovement) (Variables|/Script/Engine.Actor|GetRootComponent (Game|Player|GetPlayerPawn 0)))
  (Utilities|FlowControl|Delay 2.0)
  (Components|Activation|SetActive (Variables|Default|GetProjectileMovement) true true))

(fn ConstructionScript)