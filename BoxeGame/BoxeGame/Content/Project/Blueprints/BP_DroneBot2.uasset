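; Flying drone bot that wanders and reacts to being hit, apparently as a VR punching-bag target.
; Overlaps retune the physics constraint's angular drive, play a debounced metal sound and Niagara fireworks, and call OnPunchBag; overlap end ramps the drive stiffer via timeline.
; A looping timer drives AIMoveTo to nearby random points with slight height drift, then turns toward the player on arrival.
; Tick prints actor rotation for debugging.
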(event OnComponentBeginOverlap(DroneOverlap)
  (params (OverlappedComponent :type Primitive%20Component%20Object%20Reference) (OtherActor :type Actor%20Object%20Reference) (OtherComp :type Primitive%20Component%20Object%20Reference) (OtherBodyIndex :type Integer) (bFromSweep :type Boolean) (SweepResult :type Hit%20Result%20Structure%20%28by%20ref%29))
  (bind _returnvalue (Transformation|GetWorldLocation OtherComp))
  (bind _droneoverlap (Variables|Default|GetDroneOverlap))
  (bind _returnvalue_2 (Transformation|GetWorldLocation _droneoverlap))
  (bind _returnvalue_3 (- _returnvalue_2 _returnvalue))
  (bind _returnvalue_4 (Math|Vector|Normalize _returnvalue_3))
  (bind _returnvalue_5 (* _returnvalue_4 15.0))
  (bind _returnvalue_6 (+ _returnvalue _returnvalue_5))
  (Utilities|FlowControl|Sequence
    (:then_0
      (Audio|Components|Audio|Stop (Variables|Default|GetSlerp))
      (Class|PhysicsConstraintComponent|SetAngularDriveParams (Variables|Default|GetPhysicsConstraint) (Math|Float|MakeLiteralFloat 3e+01) (Math|Float|MakeLiteralFloat 1e+02) 0.0)
      (Utilities|FlowControl|DoOnce false
        (:Completed
          (Audio|PlaySoundatLocation "/Game/Project/Sounds/GameplaySounds/MetalSound.MetalSound" (Transformation|GetWorldLocation OtherComp) "0, 0, 0" 0.7 1.0 0.0 0 0 0)
          (Niagara|SpawnSystematLocation "/Game/Project/NiagaraAbstractSpace3/Effects/NS_Sphere_of_Fireworks.NS_Sphere_of_Fireworks" (Math|Vector|MakeVector (.x _returnvalue_6) (.y _returnvalue_6) (.z (Transformation|GetWorldLocation OtherComp)))))))
    (:then_1
      (Default|CallOnPunchBag))))

(event OnComponentEndOverlap(DroneOverlap)
  (params (OverlappedComponent :type Primitive%20Component%20Object%20Reference) (OtherActor :type Actor%20Object%20Reference) (OtherComp :type Primitive%20Component%20Object%20Reference) (OtherBodyIndex :type Integer))
  (Utilities|FlowControl|Sequence
    (:then_0
      (Utilities|FlowControl|Delay 0.5)
      (Utilities|FlowControl|DoOnce false) ; enters at Reset
    )
    (:then_1
      (bind _alpha (Timeline|Slerp PlayFromStart)
        (:Update
          (Class|PhysicsConstraintComponent|SetAngularDriveParams (Variables|Default|GetPhysicsConstraint) (Math|Float|Lerp (Math|Float|MakeLiteralFloat 1e+02) 4e+02 _alpha) (Math|Float|Lerp (Math|Float|MakeLiteralFloat 3e+01) 1.0 _alpha) 0.0))))))

(event Custom|AiMovement
  (bind _returnvalue (Transformation|GetActorLocation))
  (bind _returnvalue_2 (Transformation|GetActorLocation))
  (bind _randomlocation (AI|Navigation|GetRandomReachablePointinRadius _returnvalue 1e+02 0 0))
  (bind (_x _y) (Math|Vector|BreakVector _returnvalue_2))
  (Variables|Default|SetNewVar_0 (Math|Random|RandomFloatinRange 2.0 -2.0))
  (AI|AIMoveTo self (Math|Vector|MakeVector (.x _randomlocation) (.y _randomlocation) 0.0) 0 1.0 true
    (:then
      (Transformation|SetWorldRotation (Variables|Default|GetSkeletalMesh) (Transformation|GetActorRotation (Components|GetOwner (Variables|Character|GetCharacterMovement))) false false)
      (bind _newtrack_0 (Timeline|Timeline_2 PlayFromStart)
        (:Update
          (Transformation|SetActorLocation (Math|Vector|MakeVector _x _y (Math|Float|Lerp (.Z (Math|Vector|BreakVector (Transformation|GetActorLocation))) (+ (.Z (Math|Vector|BreakVector (Transformation|GetActorLocation))) (Variables|Default|GetNewVar_0)) _newtrack_0)) false false))))
    (:OnSuccess
      (bind _newtrack_0_2 (Timeline|Timeline_1 PlayFromStart)
        (:Update
          (Transformation|SetActorRotation (Math|Rotator|Lerp(Rotator) (Transformation|GetActorRotation) (Math|Rotator|FindLookatRotation (Transformation|GetActorLocation) (Transformation|GetActorLocation (Pawn|GetControlledPawn (Game|GetPlayerController 0)))) _newtrack_0_2 true)))))))

(event EventBeginPlay
  (bind _returnvalue (Actor|GetActorOfClass "/Game/Project/Blueprints/VRPawn.VRPawn_C"))
  (Variables|Default|SetNewVar_1 _returnvalue)
  (Class|SkeletalMeshComponent|SetAllBodiesBelowSimulatePhysics (Variables|Default|GetSkeletalMesh) (Utilities|Name|MakeLiteralName "DronBot") true true)
  (Pawn|Components|CharacterMovement|SetMovementMode (Variables|Character|GetCharacterMovement) "MOVE_Flying" 0)
  (Utilities|Time|SetTimerbyEvent (delegate Custom|AiMovement) 2.5 true 1.5))

(event Collision|EventActorBeginOverlap
  (params (OtherActor :type Actor%20Object%20Reference)))

(event EventTick
  (params (DeltaSeconds :type Float%20%28single-precision%29))
  (Development|PrintString (Utilities|String|ToString(Rotator) (Transformation|GetActorRotation)) true true "(R=0.000000,G=0.660000,B=1.000000,A=1.000000)" 0.0))

(fn ConstructionScript)