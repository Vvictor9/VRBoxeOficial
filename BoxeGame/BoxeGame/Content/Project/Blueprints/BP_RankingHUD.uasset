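; BP_RankingHUD hosts a WBP_Ranking widget in a widget component to display ranking values.
; On BeginPlay it binds to the game instance's OnAddValue event, caches the cast widget and runs its AtualizarValorRank refresh.
; AtualizarValores repeats that refresh whenever called, provided the cached widget is valid.
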(event EventBeginPlay
  (EventDispatchers|BindEventtoOnAddValue (CallFunction|GetBoxegameInstance) (EventDispatchers|CreateEvent :!event AtualizarValores))
  (bind _aswbp_ranking (Utilities|Casting|CastToWBP_Ranking (UserInterface|GetWidget (Variables|Default|GetWidget))))
  (bind _output_get (Variables|Default|SetHUD%20RankingInstance _aswbp_ranking))
  (Default|AtualizarValorRank _output_get))

(fn ConstructionScript)

(fn AtualizarValores
  (bind _hud_rankinginstance (Variables|Default|GetHUD%20RankingInstance)
    (:then
      (Default|AtualizarValorRank _hud_rankinginstance))
    (:else)))