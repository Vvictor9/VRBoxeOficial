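; VR pawn for menus that lets the player click widgets with left and right triggers.
; Each trigger sends left mouse presses and releases to its hand's WidgetInteraction component.
; BeginPlay attaches a Niagara laser to the right-hand interaction component and starts a looping timer, apparently driving the beam update.
; That update sets beam length to the hit distance over a hit-testable widget, otherwise to a short default.
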(event Custom|DestroyPointer
  (Utilities|IsValid (Variables|Default|GetPointerRef)
    (:Is%20Valid
      (Components|DestroyComponent (Variables|Default|GetPointerRef)))))

(event Custom|SpawPointer
  (bind _returnvalue (Niagara|SpawnSystemAttached "/Game/Project/Blueprints/NS_PointerLaser.NS_PointerLaser" (Variables|Default|GetWidgetInteractionR) "Pointer" "0, 0, 0" "0,0.000000, 0" "SnapToTarget" false))
  (Variables|Default|SetPointerRef _returnvalue))

(event Custom|UpdateParticlePointer
  (bind _pointerref (Variables|Default|GetPointerRef))
  (bind _widgetinteractionr (Variables|Default|GetWidgetInteractionR))
  (Utilities|IsValid _pointerref
    (:Is%20Valid
      (if (Class|WidgetInteractionComponent|IsOverHitTestVisibleWidget _widgetinteractionr)
        (Niagara|SetNiagaraVariable(Vector3) _pointerref "BeamEnd" (Math|Vector|MakeVector (.Distance (Collision|BreakHitResult (Class|WidgetInteractionComponent|GetLastHitResult _widgetinteractionr))) 0.0 0.0))
        (else
          (Niagara|SetNiagaraVariable(Vector3) _pointerref "BeamEnd" (Math|Vector|MakeVector 3e+01 0.0 0.0)))))))

(event EventBeginPlay
  (CallFunction|SpawPointer)
  (bind _returnvalue (Utilities|Time|SetTimerbyEvent (EventDispatchers|CreateEvent :!event Custom|UpdateParticlePointer) 0.1 true))
  (Variables|Default|SetTH_UpdateParticle _returnvalue))

(event Collision|EventActorBeginOverlap
  (params (OtherActor :type Actor%20Object%20Reference)))

(event EventTick
  (params (DeltaSeconds :type Float%20%28single-precision%29)))

(event Input|ActionEvents|InputActionTriggerLeft
  (params (Key :type Key%20Structure :default "None"))
  (:Pressed
    (Class|WidgetInteractionComponent|PressPointerKey (Variables|Default|GetWidgetInteractionL) "LeftMouseButton"))
  (:Released
    (Class|WidgetInteractionComponent|ReleasePointerKey (Variables|Default|GetWidgetInteractionL) "LeftMouseButton")))

(event Input|ActionEvents|InputActionTriggerRight
  (params (Key :type Key%20Structure :default "None"))
  (:Pressed
    (Class|WidgetInteractionComponent|PressPointerKey (Variables|Default|GetWidgetInteractionR) "LeftMouseButton"))
  (:Released
    (Class|WidgetInteractionComponent|ReleasePointerKey (Variables|Default|GetWidgetInteractionR) "LeftMouseButton")))

(fn ConstructionScript)